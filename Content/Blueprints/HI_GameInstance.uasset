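; Game instance serving as the shared hub for puzzle progress, level sequences and global helpers.
; Events play cinematics and looping security-bot sequences; BeginTimer runs a siren and sequence before starting BP_Timer, while background music events are empty.
; Functions track elevator fuse parts and name-keyed solved flags, though MainDoors has no setter branch.
; Other helpers toggle or destroy tagged actors, move lockdown pillars, play completion sounds and show player hints.
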(event `StartLevel1SecurityBotsSequence`
  ;[0.08369 0.3936 0.4081] SEQUENCES
  ;;[0.2051 0.9647 1] Comment
  (bind _outactor (`LevelSequencePlayer.CreateLevelSequencePlayer` (`self.LevelSecurityBot1SequencePlayer`)))
  (`MovieSceneSequencePlayer.PlayLooping` (`LevelSequenceActor.SequencePlayer` _outactor) -1)
  (bind _outactor_2 (`LevelSequencePlayer.CreateLevelSequencePlayer` (`self.LevelSecurityBot2SequencePlayer`)))
  (`MovieSceneSequencePlayer.PlayLooping` (`LevelSequenceActor.SequencePlayer` _outactor_2) -1)
  (bind _outactor_3 (`LevelSequencePlayer.CreateLevelSequencePlayer` (`self.LevelSecurityBot3SequencePlayer`)))
  (`MovieSceneSequencePlayer.PlayLooping` (`LevelSequenceActor.SequencePlayer` _outactor_3) -1)
  (bind _outactor_4 (`LevelSequencePlayer.CreateLevelSequencePlayer` (`self.LevelSecurityBot4SequencePlayer`)))
  (`MovieSceneSequencePlayer.PlayLooping` (`LevelSequenceActor.SequencePlayer` _outactor_4) -1))

(event `MoveTramSequence`
  ;[0.08369 0.3936 0.4081] SEQUENCES
  ;;[0.2051 0.9647 1] Comment
  (bind _outactor (`LevelSequencePlayer.CreateLevelSequencePlayer` (`self.LevelMoveTramSequencePlayer`)))
  (`MovieSceneSequencePlayer.Play` (`LevelSequenceActor.SequencePlayer` _outactor)))

(event `EndCreditsSequence`
  ;[0.08369 0.3936 0.4081] SEQUENCES
  ;;[0.2051 0.9647 1] Comment
  (bind _outactor (`LevelSequencePlayer.CreateLevelSequencePlayer` (`self.LevelFadeInSequencePlayer`)))
  (`MovieSceneSequencePlayer.Play` (`LevelSequenceActor.SequencePlayer` _outactor)))

(event `EndGameSequence`
  (bind _backgroundmusic (`self.BackgroundMusic`))
  ;[0.08369 0.3936 0.4081] SEQUENCES
  ;;[0.2051 0.9647 1] Comment
  (if (and (`KismetSystemLibrary.IsValid` _backgroundmusic) (`AudioComponent.IsPlaying` _backgroundmusic))
    (`AudioComponent.Stop` _backgroundmusic))
  (bind _outactor (`LevelSequencePlayer.CreateLevelSequencePlayer` (`self.LevelEndGameSequencePlayer`)))
  (`MovieSceneSequencePlayer.Play` (`LevelSequenceActor.SequencePlayer` _outactor)))

(event `BackgroundMusicLevel01`
  ;[1 0.06126 0.3631] BackgroundMusic
)

(event `BackgroundMusicLevel02`
  ;[1 0.06126 0.3631] BackgroundMusic
)

(event `LevelFadeInSequence`
  ;[0.08369 0.3936 0.4081] SEQUENCES
  ;;[0.2051 0.9647 1] Comment
  (bind _outactor (`LevelSequencePlayer.CreateLevelSequencePlayer` (`self.LevelFadeInSequencePlayer`)))
  (`MovieSceneSequencePlayer.Play` (`LevelSequenceActor.SequencePlayer` _outactor)))

(event `LevelFadeOutSequence`
  ;[0.08369 0.3936 0.4081] SEQUENCES
  ;;[0.2051 0.9647 1] Comment
  (bind _outactor (`LevelSequencePlayer.CreateLevelSequencePlayer` (`self.LevelFadeOutSequencePlayer`)))
  (`MovieSceneSequencePlayer.Play` (`LevelSequenceActor.SequencePlayer` _outactor)))

(event `BeginTimer`
  ;[0 0 0] Begin Timer
  (`KismetSystemLibrary.Delay` 2.0)
  (bind _returnvalue (`GameplayStatics.SpawnSound2D` null 0.3 1.0 0.0 null))
  (set `self.SirenSound` _returnvalue)
  (bind _outactor (`LevelSequencePlayer.CreateLevelSequencePlayer` (`self.SequencePlayer`)))
  (`MovieSceneSequencePlayer.Play` (`LevelSequenceActor.SequencePlayer` _outactor))
  (`KismetSystemLibrary.Delay` 4.0)
  (`KismetSystemLibrary.Delay` 1.0)
  (`AudioComponent.Stop` (`self.SirenSound`))
  (bind _returnvalue_2 (`GameplayStatics.GetActorOfClass` "/Game/Blueprints/Actors/Interaction/BP_Timer.BP_Timer_C"))
  (`/Game/Blueprints/Actors/Interaction/BP_Timer.BeginTimer` _returnvalue_2))

(fn `CollectFusePart`
  (bind _elevatorfusepartstotalneeded (`self.elevatorFusePartsTotalNeeded`))
  (bind _output_get (set `self.elevatorFusePartsCarrying` (+ (`self.elevatorFusePartsCarrying`) 1)))
  (bind _returnvalue (+ _output_get (`self.elevatorFusePartsInserted`)))
  (if (== _returnvalue _elevatorfusepartstotalneeded)
    (`KismetSystemLibrary.PrintString` "Found all the fuses, now put them in the elevator fuse box")
    (else
      (`KismetSystemLibrary.PrintString` "Still need")
      (`KismetSystemLibrary.PrintString` (`KismetStringLibrary.Conv_IntToString` (- _elevatorfusepartstotalneeded _returnvalue))))))

(fn `GetHasSolved`
  (params (VariableName :type String))
  (returns (HasSolved :type Boolean))
  (if (`KismetStringLibrary.EqualEqual_StrStr` VariableName "ElectricalPanelSmall")
    (return (`self.hasSolvedElectricalPanelSmall`))
    (elif (`KismetStringLibrary.EqualEqual_StrStr` VariableName "ElectricalPanel")
      (return (`self.hasSolvedElectricalPanel`))
      (elif (`KismetStringLibrary.EqualEqual_StrStr` VariableName "SecurityLasers")
        (return (`self.hasSolvedSecurityLasers`))
        (elif (`KismetStringLibrary.EqualEqual_StrStr` VariableName "ElevatorPuzzle")
          (return (`self.hasSolvedElevatorPuzzle`))
          (elif (`KismetStringLibrary.EqualEqual_StrStr` VariableName "SparkPlugPuzzleSimple")
            (return (`self.hasSolvedSparkPlugPuzzleSimple`))
            (elif (`KismetStringLibrary.EqualEqual_StrStr` VariableName "SparkPlugPuzzle")
              (return (`self.hasSolvedSparkPlugPuzzle`))
              (elif (`KismetStringLibrary.EqualEqual_StrStr` VariableName "MainDoors")
                (return (`self.hasUnlockedMainDoors`))
                (else
                  (return false))))))))))

(fn `HideActorsByTag`
  (params (tag :type String) (destroyActor :type Boolean))
  (bind _outactors (`GameplayStatics.GetAllActorsWithTag` (`KismetStringLibrary.Conv_StringToName` tag)))
  (for _array_element _outactors
    (if destroyActor
      (`Actor.K2_DestroyActor` _array_element)
      (else
        (`SceneComponent.SetVisibility` (`Actor.RootComponent` _array_element) false false)))))

(fn `InitiateSecurityPillar`
  (params (PillarTag :type String))
  (bind _outactors (`GameplayStatics.GetAllActorsOfClassWithTag` "/Game/Blueprints/Actors/Movement/BP_LockdownPillars.BP_LockdownPillars_C" (`KismetStringLibrary.Conv_StringToName` PillarTag)))
  (for _array_element _outactors
    (`/Game/Blueprints/Actors/Movement/BP_LockdownPillars.MovePillar` _array_element)))

(fn `InsertFusePart`
  (returns (newFusePartsCarrying :type Integer) (newFusePartsInserted :type Integer) (solvedPuzzle :type Boolean))
  ;[0.4068 1 0.4825] Comment
  (if (> (`self.elevatorFusePartsCarrying`) 0)
    (bind _output_get (set `self.elevatorFusePartsCarrying` (- (`self.elevatorFusePartsCarrying`) 1)))
    (bind _output_get_2 (set `self.elevatorFusePartsInserted` (+ (`self.elevatorFusePartsInserted`) 1)))
    (if (>= _output_get_2 (`self.elevatorFusePartsTotalNeeded`))
      (set `self.hasSolvedElevatorPuzzle` true))
    (return (`self.elevatorFusePartsCarrying`) (`self.elevatorFusePartsInserted`) (`self.hasSolvedElevatorPuzzle`))))

(fn `SetHasSolved`
  (params (VariableName :type String) (HasSolved :type Boolean))
  (if (`KismetStringLibrary.EqualEqual_StrStr` VariableName "ElectricalPanelSmall")
    (set `self.hasSolvedElectricalPanelSmall` HasSolved)
    (elif (`KismetStringLibrary.EqualEqual_StrStr` VariableName "ElectricalPanel")
      (set `self.hasSolvedElectricalPanel` HasSolved)
      (elif (`KismetStringLibrary.EqualEqual_StrStr` VariableName "SecurityLasers")
        (set `self.hasSolvedSecurityLasers` HasSolved)
        (elif (`KismetStringLibrary.EqualEqual_StrStr` VariableName "ElevatorPuzzle")
          (set `self.hasSolvedElevatorPuzzle` HasSolved)
          (elif (`KismetStringLibrary.EqualEqual_StrStr` VariableName "SparkPlugPuzzleSimple")
            (set `self.hasSolvedSparkPlugPuzzleSimple` HasSolved)
            (elif (`KismetStringLibrary.EqualEqual_StrStr` VariableName "SparkPlugPuzzle")
              (set `self.hasSolvedSparkPlugPuzzle` HasSolved))))))))

(fn `ShowActorsByTag`
  (params (tag :type String))
  (bind _outactors (`GameplayStatics.GetAllActorsWithTag` (`KismetStringLibrary.Conv_StringToName` tag)))
  (for _array_element _outactors
    (`SceneComponent.SetVisibility` (`Actor.RootComponent` _array_element) true false)))

(fn `ShowMessageUI`
  (params (Message :type Text))
  (bind _asbp_hiplayer_char (cast `/Game/Blueprints/Characters/PC/BP_HIPlayerChar` (`GameplayStatics.GetPlayerCharacter` 0)))
  (`/Game/UI/WBP_UserHints.SetUserMessage` (`/Game/Blueprints/Characters/PC/BP_HIPlayerChar.UserHintsWidget` _asbp_hiplayer_char) Message))

(fn `TaskComplete`
  (`|ExecutionSequence`
    (:`then_0`
      (`GameplayStatics.PlaySound2D` null 0.25 1.0 0.0 null null))
    (:`then_1`
      (`GameplayStatics.PlaySound2D` null 1.0 1.0 0.7 null null))))