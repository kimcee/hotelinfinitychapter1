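; Planetarium star generator that builds a night sky from a star catalog DataTable on BeginPlay or SpawnNow.
; GenerateStars clears and refills one instanced mesh component per spectral class for color, stopping at the Amount fraction of rows.
; Right ascension and declination place stars at a fixed radius, rotated toward a look-at target, with magnitude driving scale through an exponent curve.
; Debug helpers find stars by Hipparcos number or index, drawing lines and printing details.
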(event `SpawnNow`
  (`/Engine/EditorBlueprintResources/StandardMacros.DoOnce` false :!label _label
    (:`Completed`
      (bind _outrownames (`DataTableFunctionLibrary.GetDataTableRowNames` (`self.DataTable`)))
      (set `self.Data` _outrownames)
      (`self.GenerateStars`)
      (`|ExecutionSequence`
        (:`then_0`
          (goto _label :!via `Reset`))))))

(event `self.ReceiveBeginPlay`
  (bind _outrownames (`DataTableFunctionLibrary.GetDataTableRowNames` (`self.DataTable`)))
  (set `self.Data` _outrownames)
  (`self.GenerateStars`))

(event `GenerateStars`
  (bind _data (`self.Data`))
  (`InstancedStaticMeshComponent.ClearInstances` (`self.StarsO`)) ; destroy existing stars
  (`InstancedStaticMeshComponent.ClearInstances` (`self.StarsB`))
  (`InstancedStaticMeshComponent.ClearInstances` (`self.StarsA`))
  (`InstancedStaticMeshComponent.ClearInstances` (`self.StarsF`))
  (`InstancedStaticMeshComponent.ClearInstances` (`self.StarsG`))
  (`InstancedStaticMeshComponent.ClearInstances` (`self.StarsK`))
  (`InstancedStaticMeshComponent.ClearInstances` (`self.StarsM`))
  (for (_array_element _array_index) _data
    (if (> (`KismetMathLibrary.NormalizeToRange` (`KismetMathLibrary.Conv_IntToDouble` _array_index) 0.0 (`KismetMathLibrary.Conv_IntToDouble` (`KismetArrayLibrary.Array_LastIndex` _data))) (`self.Amount`))
      (break)
      (else
        (bind _returnvalue (`|GetDataTableRow` (`self.DataTable`) _array_element)
          (:`then`
            (bind (_ra _dec _dist _mag _spect) (break `/Game/Blueprints/Environment/StructStars` _returnvalue))
            (bind _returnvalue_2 (* (`KismetMathLibrary.GetForwardVector` (`KismetMathLibrary.MakeRotator` 0.0 _dec (* -15 _ra))) (`self.PlanetariumScale`)))
            (set `self.CurrentInstLoc` _returnvalue_2)
            (set `self.CurrentInstRot` (`KismetMathLibrary.FindLookAtRotation` _returnvalue_2 (`self.K2_GetActorLocation`))) ; Rotate star plane to Generator location
            (set `self.CurrentInstScale` (`KismetMathLibrary.Conv_DoubleToVector` (* (`KismetMathLibrary.MultiplyMultiply_FloatFloat` (`KismetMathLibrary.MapRangeClamped` _mag 10.0 -1.5 (`self.SmallestStar`) (`self.LargestStar`)) (`self.Exponent`)) (`self.StarScale`))))
            (switch `string` (`KismetStringLibrary.Left` _spect 1) ; Spectral Class determines Star Color
              (:`Default`
                (`InstancedStaticMeshComponent.AddInstance` (`self.StarsG`) (`KismetMathLibrary.MakeTransform` (`self.CurrentInstLoc`) (`self.CurrentInstRot`) (`self.CurrentInstScale`)) false :!label _label_2))
              (:`O`
                (`InstancedStaticMeshComponent.AddInstance` (`self.StarsO`) (`KismetMathLibrary.MakeTransform` (`self.CurrentInstLoc`) (`self.CurrentInstRot`) (`self.CurrentInstScale`)) false))
              (:`B`
                (`InstancedStaticMeshComponent.AddInstance` (`self.StarsB`) (`KismetMathLibrary.MakeTransform` (`self.CurrentInstLoc`) (`self.CurrentInstRot`) (`self.CurrentInstScale`)) false))
              (:`A`
                (`InstancedStaticMeshComponent.AddInstance` (`self.StarsA`) (`KismetMathLibrary.MakeTransform` (`self.CurrentInstLoc`) (`self.CurrentInstRot`) (`self.CurrentInstScale`)) false))
              (:`F`
                (`InstancedStaticMeshComponent.AddInstance` (`self.StarsF`) (`KismetMathLibrary.MakeTransform` (`self.CurrentInstLoc`) (`self.CurrentInstRot`) (`self.CurrentInstScale`)) false))
              (:`G`
                (goto _label_2))
              (:`K`
                (`InstancedStaticMeshComponent.AddInstance` (`self.StarsK`) (`KismetMathLibrary.MakeTransform` (`self.CurrentInstLoc`) (`self.CurrentInstRot`) (`self.CurrentInstScale`)) false))
              (:`M`
                (`InstancedStaticMeshComponent.AddInstance` (`self.StarsM`) (`KismetMathLibrary.MakeTransform` (`self.CurrentInstLoc`) (`self.CurrentInstRot`) (`self.CurrentInstScale`)) false)))))))))

(event `FindStar`
  (params (Hipparcos :type Integer))
  ;[0 0 0] Find Star by Hipparcos number
  (for (_array_element _array_index) (`self.Data`)
    (bind _returnvalue (`|GetDataTableRow` (`self.DataTable`) _array_element)
      (:`then`
        (bind (_ra _dec _dist _mag _spect _ci _x _y _z _lum _proper _hip) (break `/Game/Blueprints/Environment/StructStars` _returnvalue))
        (if (== _hip Hipparcos)
          (`KismetSystemLibrary.PrintString` (`KismetStringLibrary.Concat_StrStr` "HIP " (`KismetStringLibrary.Conv_IntToString` _hip)) true true (struct :`G` 0.66 :`B` 1.0 :`A` 1.0) 10.0)
          (`self.PointStarAtIndex` _array_index) ; Polaris
          (break))))))

(fn `PointStarAtIndex`
  (params (Index :type Integer))
  (bind _returnvalue (`self.K2_GetActorLocation`))
  (bind _returnvalue_2 (`|GetDataTableRow` (`self.DataTable`) (`|GetArrayItem` (`self.Data`) Index))
    (:`then`
      (bind (_ra _dec _dist _mag _spect _ci _x _y _z _lum _proper) (break `/Game/Blueprints/Environment/StructStars` _returnvalue_2))
      (`KismetSystemLibrary.DrawDebugLine` _returnvalue (+ _returnvalue (* (`KismetMathLibrary.GetForwardVector` (`KismetMathLibrary.MakeRotator` 0.0 _dec (* -15 _ra))) (`self.PlanetariumScale`))) (struct :`R` 1.0 :`A` 1.0) 20.0 5.0)
      (`KismetSystemLibrary.PrintString` _proper true true (struct :`G` 0.66 :`B` 1.0 :`A` 1.0) 20.0)
      (`KismetSystemLibrary.PrintString` (`KismetStringLibrary.Concat_StrStr` "RA: " (`KismetStringLibrary.Conv_DoubleToString` _ra) "| Dec: " (`KismetStringLibrary.Conv_DoubleToString` _dec) "| Dist: " (`KismetStringLibrary.Conv_DoubleToString` _dist) "| Class: " _spect) true true (struct :`G` 0.66 :`B` 1.0 :`A` 1.0) 20.0))))

(fn `SetStarScale`
  (params (Scale :type "Float (double-precision)"))
  (set `self.StarScale` Scale))

(fn `UserConstructionScript`)