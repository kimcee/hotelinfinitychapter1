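; Security laser actor that sweeps its laser component back and forth along its local Y axis until the security laser puzzle is solved.
; After a configurable start delay, a self-calling LoopAction event alternately plays and reverses a Timeline that lerps the relative location, pausing between halves.
; Tick polls HI_GameInstance for the solved flag, then deactivates the loop and destroys the laser component.
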(event `self.ReceiveTick`
  (params (DeltaSeconds :type "Float (single-precision)"))
  ;[1 0.7959 0.5005] Event Tick
  (if (`self.isActive`)
    (bind _ashi_game_instance (cast `/Game/Blueprints/HI_GameInstance` (`GameplayStatics.GetGameInstance`)))
    (if (`/Game/Blueprints/HI_GameInstance.hasSolvedSecurityLasers` _ashi_game_instance)
      (`self.DisableLazer`))))

(event `self.ReceiveBeginPlay`
  ;[1 1 1] Begin
  (`KismetSystemLibrary.Delay` (`self.DelayStartTime`))
  (`self.LoopAction`))

(event `LoopAction`
  (bind _delaybetweenanimationtime (`self.DelayBetweenAnimationTime`))
  ;[1 0.2494 0.8493] Recursive Loop
  (if (`self.isActive`)
    (`self.FirstHalf`)
    (`KismetSystemLibrary.Delay` _delaybetweenanimationtime)
    (`self.SecondHalf`)
    (`KismetSystemLibrary.Delay` _delaybetweenanimationtime)
    (`self.LoopAction`)))

(event `FirstHalf`
  ;[0.2128 0.6041 1] Animation
  (if (`self.isActive`)
    (bind (_direction _alpha) (`Timeline|Timeline` :!label _label)
      (:`Update`
        (`SceneComponent.K2_SetRelativeLocation` (`self.BP_Lazer`) (`KismetMathLibrary.MakeVector` 0.0 (`KismetMathLibrary.Lerp` 0.0 1000.0 _alpha)) false false)))))

(event `SecondHalf`
  ;[0.2128 0.6041 1] Animation
  (if (`self.isActive`)
    (goto _label :!via `Reverse`)))

(event `DisableLazer`
  ;[1 1 1] Comment
  (set `self.isActive` false)
  (`ActorComponent.K2_DestroyComponent` (`self.BP_Lazer`)))

(fn `UserConstructionScript`)