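; BP_LazerMoveIntoPlace is a laser hazard that waits offset from its active position and kills the player on contact.
; BeginPlay and ResetLazer offset the Lazer component vertically by DistanceToMove, below or above according to HideBelow.
; MoveIntoPlace snaps it back to its relative origin without interpolation.
; Box overlap with BP_HIPlayerChar finds the BP_Timer actor and calls KillPlayerDuringTimerRun on it.
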(event `self.ReceiveBeginPlay`
  (if (`self.HideBelow`) :!label _label
    (`SceneComponent.K2_SetRelativeLocation` (`self.Lazer`) (`KismetMathLibrary.MakeVector` 0.0 0.0 (* (`self.DistanceToMove`) -1.0)) false false)
    (else
      (`SceneComponent.K2_SetRelativeLocation` (`self.Lazer`) (`KismetMathLibrary.MakeVector` 0.0 0.0 (`self.DistanceToMove`)) false false))))

(event `ResetLazer`
  (goto _label))

(event `MoveIntoPlace`
  (`SceneComponent.K2_SetRelativeLocation` (`self.Lazer`) (0.0 0.0 0.0) false false))

(event `self.Box.OnComponentBeginOverlap`
  (params (OverlappedComponent :type "PrimitiveComponent Object Reference") (OtherActor :type "Actor Object Reference") (OtherComp :type "PrimitiveComponent Object Reference") (OtherBodyIndex :type Integer) (bFromSweep :type Boolean) (SweepResult :type "HitResult Structure (by ref)"))
  (cast `/Game/Blueprints/Characters/PC/BP_HIPlayerChar` OtherActor)
  (bind _returnvalue (`GameplayStatics.GetActorOfClass` "/Game/Blueprints/Actors/Interaction/BP_Timer.BP_Timer_C"))
  (`/Game/Blueprints/Actors/Interaction/BP_Timer.KillPlayerDuringTimerRun` _returnvalue))

(fn `UserConstructionScript`)