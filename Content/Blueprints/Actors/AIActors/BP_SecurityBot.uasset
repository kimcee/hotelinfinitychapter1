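; BP_SecurityBot is a sweeping security sentry that kills the player on contact with its collision volume.
; After a start delay, a recursive event loop plays and reverses a timeline, with pauses, to yaw its cube back and forth.
; On overlap, the L1_Character is spared only if also overlapping a TriggerBox actor.
; Tick polls the game instance's laser-puzzle flag, then deactivates the bot, destroying its collision and lights.
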(event `self.ReceiveTick`
  (params (DeltaSeconds :type "Float (single-precision)"))
  ;[1 0.7959 0.5005] Event Tick
  (if (`self.isActive`)
    (bind _ashi_game_instance (cast `/Game/Blueprints/HI_GameInstance` (`GameplayStatics.GetGameInstance`)))
    (if (`/Game/Blueprints/HI_GameInstance.hasSolvedSecurityLasers` _ashi_game_instance)
      (`self.DisableBot`))))

(event `self.ReceiveBeginPlay`
  ;[1 1 1] Begin
  (`KismetSystemLibrary.Delay` (`self.DelayStartTime`))
  (`self.LoopAction`))

(event `LoopAction`
  (bind _delaybetweenanimationtime (`self.DelayBetweenAnimationTime`))
  ;[1 0.2494 0.8493] Recursive Loop
  (if (`self.isActive`)
    (`self.FirstHalf`)
    (`KismetSystemLibrary.Delay` _delaybetweenanimationtime)
    (`self.SecondHalf`)
    (`KismetSystemLibrary.Delay` _delaybetweenanimationtime)
    (`self.LoopAction`)))

(event `FirstHalf`
  ;[0.2128 0.6041 1] Animation
  (bind (_direction _newtrack_0) (`Timeline|Timeline_0` :!label _label)
    (:`Update`
      (`SceneComponent.K2_SetRelativeRotation` (`self.Cube1`) (`KismetMathLibrary.MakeRotator` 0.0 0.0 (`KismetMathLibrary.Lerp` (`self.StartRotation`) (`self.MaxRotation`) _newtrack_0)) false false))))

(event `SecondHalf`
  ;[0.2128 0.6041 1] Animation
  (goto _label :!via `Reverse`))

(event `self.Collision.OnComponentBeginOverlap`
  (params (OverlappedComponent :type "PrimitiveComponent Object Reference") (OtherActor :type "Actor Object Reference") (OtherComp :type "PrimitiveComponent Object Reference") (OtherBodyIndex :type Integer) (bFromSweep :type Boolean) (SweepResult :type "HitResult Structure (by ref)"))
  ;[1 1 1] Trigger
  (bind _asl1_character (cast `/Game/Blueprints/Level1/L1_Character` OtherActor))
  (set `self.isPlayerSafe` false)
  (for _array_element (`self.GetOverlappingActors` _asl1_character null)
    (if (`KismetStringLibrary.EqualEqual_StrStr` (`KismetSystemLibrary.GetClassDisplayName` (`GameplayStatics.GetObjectClass` _array_element)) "TriggerBox")
      (set `self.isPlayerSafe` true)))
  (if (not (`self.isPlayerSafe`))
    (`/Game/Blueprints/Level1/L1_Character.KillPlayer` _asl1_character)))

(fn `DisableBot`
  (set `self.isActive` false)
  (`ActorComponent.K2_DestroyComponent` (`self.Collision`))
  (`ActorComponent.K2_DestroyComponent` (`self.PointLight`))
  (`ActorComponent.K2_DestroyComponent` (`self.SpotLight`)))

(fn `UserConstructionScript`)