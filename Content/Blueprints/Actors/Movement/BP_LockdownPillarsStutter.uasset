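; Lockdown pillar actor that raises, gradually lowers and fully closes its static mesh using three timelines driving relative Z.
; OpenPillar plays a door sound and lifts the mesh.
; The first L1_Character overlap after HI_GameInstance flags the spark plug puzzle solved starts MovePillar, lowering it most of the way.
; ClosePillar, not called here, halts that movement, drops the mesh to zero and plays an explosion sound on finish.
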(event `OpenPillar`
  ;[1 0.3314 0] Open Pillar
  (`GameplayStatics.PlaySoundAtLocation` "/Game/Audio/large_door_open.large_door_open" (`self.K2_GetActorLocation` (`ActorComponent.GetOwner` (`self.StaticMesh`))) (struct) 1.0 1.0 0.0 null null null null)
  (bind (_direction _alpha) (`Timeline|OpenPillarTL`)
    (:`Update`
      (`SceneComponent.K2_SetRelativeLocation` (`self.StaticMesh`) (`KismetMathLibrary.MakeVector` 0.0 0.0 (`KismetMathLibrary.Lerp` 0.0 500.0 _alpha)) false false))))

(event `MovePillar`
  ;[1 0.194 0.8936] Begin to Close Pillar
  (bind (_direction _alpha) (`Timeline|MovementTL`)
    (:`Update`
      (`SceneComponent.K2_SetRelativeLocation` (`self.StaticMesh`) (`KismetMathLibrary.MakeVector` 0.0 0.0 (`KismetMathLibrary.Lerp` 500.0 100.0 _alpha)) false false))))

(event `ClosePillar`
  ;[0.1305 0.3675 1] Close Pillar
  (`TimelineComponent.Stop` (`self.MovementTL`))
  (bind (_direction _alpha) (`Timeline|ClosePillarTL`)
    (:`Update`
      (`SceneComponent.K2_SetRelativeLocation` (`self.StaticMesh`) (`KismetMathLibrary.MakeVector` 0.0 0.0 (`KismetMathLibrary.Lerp` 100.0 0.0 _alpha)) false false))
    (:`Finished`
      (`GameplayStatics.PlaySoundAtLocation` "/Game/StarterContent/Audio/Explosion02.Explosion02" (`SceneComponent.K2_GetComponentLocation` (`self.StaticMesh`)) (struct) 1.0 1.0 0.0 null null null null))))

(event `self.Collision.OnComponentBeginOverlap`
  (params (OverlappedComponent :type "PrimitiveComponent Object Reference") (OtherActor :type "Actor Object Reference") (OtherComp :type "PrimitiveComponent Object Reference") (OtherBodyIndex :type Integer) (bFromSweep :type Boolean) (SweepResult :type "HitResult Structure (by ref)"))
  ;[0 0 0] Activate Close Pillar
  (cast `/Game/Blueprints/Level1/L1_Character` OtherActor)
  (bind _ashi_game_instance (cast `/Game/Blueprints/HI_GameInstance` (`GameplayStatics.GetGameInstance`)))
  (if (`/Game/Blueprints/HI_GameInstance.hasSolvedSparkPlugPuzzle` _ashi_game_instance)
    (if (not (`self.hasMoved`))
      (set `self.hasMoved` true)
      (`self.MovePillar`))))

(fn `UserConstructionScript`)