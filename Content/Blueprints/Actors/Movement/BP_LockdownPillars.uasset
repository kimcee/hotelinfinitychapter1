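; BP_LockdownPillars is a pillar that moves vertically when the player enters its collision after the spark plug puzzle is solved.
; The overlap checks CanInteract and the game instance's puzzle flag, then calls MovePillar once, guarded by HasMoved.
; The Movement timeline lerps the mesh's relative Z from DistanceToMove to zero, playing a sound on arrival.
; ResetPillar clears HasMoved and reverses the timeline from its end.
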(event `MovePillar`
  (set `self.hasMoved` true)
  (bind (_direction _alpha) (`Timeline|Movement` :!label _label)
    (:`Update`
      (`SceneComponent.K2_SetRelativeLocation` (`self.StaticMesh`) (`KismetMathLibrary.MakeVector` 0.0 0.0 (`KismetMathLibrary.Lerp` (`self.DistanceToMove`) 0.0 _alpha)) false false))
    (:`Finished`
      (if (`self.hasMoved`)
        (`GameplayStatics.PlaySoundAtLocation` null (`SceneComponent.K2_GetComponentLocation` (`self.StaticMesh`)) (struct) 1.0 1.0 0.0 null null null null)))))

(event `ResetPillar`
  (if (`self.hasMoved`)
    (set `self.hasMoved` false)
    (goto _label :!via `ReverseFromEnd`)))

(event `self.Collision.OnComponentBeginOverlap`
  (params (OverlappedComponent :type "PrimitiveComponent Object Reference") (OtherActor :type "Actor Object Reference") (OtherComp :type "PrimitiveComponent Object Reference") (OtherBodyIndex :type Integer) (bFromSweep :type Boolean) (SweepResult :type "HitResult Structure (by ref)"))
  (cast `/Game/Blueprints/Characters/PC/BP_HIPlayerChar` OtherActor)
  (if (`self.canInteract`)
    (bind _ashi_game_instance (cast `/Game/Blueprints/HI_GameInstance` (`GameplayStatics.GetGameInstance`)))
    (if (`/Game/Blueprints/HI_GameInstance.hasSolvedSparkPlugPuzzle` _ashi_game_instance)
      (if (not (`self.hasMoved`))
        (set `self.hasMoved` true)
        (bind _ashi_game_instance_2 (cast `/Game/Blueprints/HI_GameInstance` (`GameplayStatics.GetGameInstance`)))
        (if (`/Game/Blueprints/HI_GameInstance.hasSolvedSparkPlugPuzzle` _ashi_game_instance_2)
          (`self.MovePillar`))))))

(fn `UserConstructionScript`)