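; Interaction actor for the flashlight pickup, which grants the player the flashlight.
; On BeginPlay it destroys itself if the game instance already records HasFlashLight, otherwise it runs parent setup.
; Interact sets that flag, plays a pickup sound, hides the cube and outline, and shows the toggle-key message through the game instance.
; The actor is destroyed after a short delay.
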(event `self.ReceiveBeginPlay`
  (bind _ashi_game_instance (cast `/Game/Blueprints/HI_GameInstance` (`GameplayStatics.GetGameInstance`)))
  (if (`/Game/Blueprints/HI_GameInstance.hasFlashLight` _ashi_game_instance)
    (`self.K2_DestroyActor`)
    (else
      (`parent.ReceiveBeginPlay`))))

(event `/Game/Blueprints/Interfaces/BPI_Interaction.Interact`
  (bind _ashi_game_instance (cast `/Game/Blueprints/HI_GameInstance` (`GameplayStatics.GetGameInstance`)))
  (set `/Game/Blueprints/HI_GameInstance.hasFlashLight` true _ashi_game_instance)
  (`GameplayStatics.PlaySound2D` "/Engine/VREditor/Sounds/UI/Object_PickUp.Object_PickUp" 1.0 1.0 0.0 null null)
  (`SceneComponent.SetVisibility` (`self.Cube`) false false)
  (`SceneComponent.SetVisibility` (`self.OutlineCollision`) false false)
  (`/Game/Blueprints/HI_GameInstance.ShowMessageUI` _ashi_game_instance "Press \"F\" to Toggle Flashlight")
  (`KismetSystemLibrary.Delay` 4.0)
  (`self.K2_DestroyActor`))

(fn `UserConstructionScript`
  (`parent.UserConstructionScript`))