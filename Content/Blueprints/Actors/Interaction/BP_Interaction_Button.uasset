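; Interactable button that marks the electrical panel puzzle as solved.
; On Interact it sets the solved flag on HI_GameInstance, clears focus on the BP_Interaction_PuzzleFocus actor, then toggles between error and success visuals.
; The toggle swaps error and success light visibility, with error particles following the error light.
; BeginPlay reuses the error branch to start in the error state, bypassing the light validity check.
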(event `/Game/Blueprints/Interfaces/BPI_Interaction.Interact`
  (bind _errorlight (`self.ErrorLight`))
  (bind _lightcomponent (`Light.LightComponent` (`self.SuccessLight`)))
  (bind _lightcomponent_2 (`Light.LightComponent` _errorlight))
  (bind _particlesystemcomponent (`Emitter.ParticleSystemComponent` (`self.ErrorParticles`)))
  (bind _ashi_game_instance (cast `/Game/Blueprints/HI_GameInstance` (`GameplayStatics.GetGameInstance`)))
  (set `/Game/Blueprints/HI_GameInstance.hasSolvedElectricalPanel` true _ashi_game_instance)
  ;[1 1 1] Reset Character Movement
  (bind _returnvalue (`GameplayStatics.GetActorOfClass` "/Game/Blueprints/Actors/Interaction/BP_Interaction_PuzzleFocus.BP_Interaction_PuzzleFocus_C"))
  (set `/Game/Blueprints/Actors/Interaction/BP_Interaction_PuzzleFocus.isFocused` false _returnvalue)
  (`/Engine/EditorBlueprintResources/StandardMacros.IsValid` _errorlight
    (:`Is Valid`
      (if (`SceneComponent.bVisible` _lightcomponent_2)
        (`SceneComponent.SetVisibility` _lightcomponent_2 false false)
        (`SceneComponent.SetVisibility` _lightcomponent true false)
        (`SceneComponent.SetVisibility` _particlesystemcomponent false false)
        (else
          (`SceneComponent.SetVisibility` _lightcomponent_2 true false :!label _label)
          (`SceneComponent.SetVisibility` _lightcomponent false false)
          (`SceneComponent.SetVisibility` _particlesystemcomponent true false))))))

(event `self.ReceiveBeginPlay`
  (goto _label))

(fn `UserConstructionScript`
  (`parent.UserConstructionScript`))