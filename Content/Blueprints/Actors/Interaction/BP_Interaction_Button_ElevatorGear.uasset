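; Elevator gear interaction that lets the player insert carried fuses to solve the elevator fuse puzzle.
; Interacting blends to the fuse camera, then a delayed recursive event reveals hidden "fusePart" actors one at a time while HI_GameInstance reports fuses carried.
; Once solved, it returns the camera, swaps tagged actors, completes the task, disables itself and switches the elevator light to success.
; Otherwise, messages prompt the player to find fuses.
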(event `/Game/Blueprints/Interfaces/BPI_Interaction.Interact`
  ;[1 0.1869 0.7907] Comment
  (bind _ashi_game_instance (cast `/Game/Blueprints/HI_GameInstance` (`GameplayStatics.GetGameInstance`)))
  (if (> (`/Game/Blueprints/HI_GameInstance.elevatorFusePartsCarrying` _ashi_game_instance) 0)
    (`self.MoveToCamera`)
    (`KismetSystemLibrary.Delay` 1.0)
    (`self.AddFusePart`)
    (else
      (`/Game/Blueprints/HI_GameInstance.ShowMessageUI` _ashi_game_instance "Find Missing Fuses"))))

(event `MoveToCamera`
  ;[0.9325 1 0.2783] Comment
  (bind _returnvalue (`GameplayStatics.GetActorOfClass` "/Game/Blueprints/Cameras/BP_BlendTriggerVolume.BP_BlendTriggerVolume_C"))
  (if (not (`/Game/Blueprints/Cameras/BP_BlendTriggerVolume.isFocused` _returnvalue))
    (bind _returnvalue_2 (`GameplayStatics.GetActorOfClass` "/Game/Blueprints/Cameras/BP_CameraElevatorFuses.BP_CameraElevatorFuses_C"))
    (`/Game/Blueprints/Cameras/BP_BlendTriggerVolume.MoveToCamera` _returnvalue _returnvalue_2)))

(event `AddFusePart`
  ;[0.4136 1 0.5924] Comment
  (`KismetSystemLibrary.Delay` 0.25)
  (bind _ashi_game_instance (cast `/Game/Blueprints/HI_GameInstance` (`GameplayStatics.GetGameInstance`)))
  (if (> (`/Game/Blueprints/HI_GameInstance.elevatorFusePartsCarrying` _ashi_game_instance) 0)
    (bind _outactors (`GameplayStatics.GetAllActorsWithTag` "fusePart"))
    (for _array_element _outactors
      (bind _asbp_interaction_fuse (cast `/Game/Blueprints/Actors/Interaction/BP_Interaction_Fuse` _array_element))
      (if (`/Game/Blueprints/Actors/Interaction/BP_Interaction_Fuse.isHidden` _asbp_interaction_fuse)
        (`/Game/Blueprints/HI_GameInstance.InsertFusePart` _ashi_game_instance)
        (`/Game/Blueprints/Actors/Interaction/BP_Interaction_Fuse.InsertPart` _asbp_interaction_fuse)
        (break)))
    (if (> (`/Game/Blueprints/HI_GameInstance.elevatorFusePartsCarrying` _ashi_game_instance) 0)
      (`self.AddFusePart`)
      (else
        (`self.CheckForAllFusePartsInserted`)))))

(event `CheckForAllFusePartsInserted`
  ;[1 1 1] Comment
  (`KismetSystemLibrary.Delay` 0.5)
  (bind _ashi_game_instance (cast `/Game/Blueprints/HI_GameInstance` (`GameplayStatics.GetGameInstance`)))
  (if (`/Game/Blueprints/HI_GameInstance.hasSolvedElevatorPuzzle` _ashi_game_instance)
    (bind _returnvalue (`GameplayStatics.GetActorOfClass` "/Game/Blueprints/Cameras/BP_BlendTriggerVolume.BP_BlendTriggerVolume_C"))
    (`/Game/Blueprints/Cameras/BP_BlendTriggerVolume.ReturnToCharacter` _returnvalue)
    (`/Game/Blueprints/HI_GameInstance.HideActorsByTag` _ashi_game_instance (`self.HideByTag`) true)
    (`/Game/Blueprints/HI_GameInstance.ShowActorsByTag` _ashi_game_instance (`self.ShowByTag`))
    (`/Game/Blueprints/HI_GameInstance.TaskComplete` _ashi_game_instance)
    (`ActorComponent.K2_DestroyComponent` (`self.OutlineCollision`))
    (`Widget.SetVisibility` (`self.InteractWidget`) "Hidden")
    (bind _returnvalue_2 (`GameplayStatics.GetActorOfClass` "/Game/Blueprints/Actors/Interaction/BP_Interaction_Elevator.BP_Interaction_Elevator_C"))
    (`SceneComponent.SetVisibility` (`/Game/Blueprints/Actors/Interaction/BP_Interaction_Elevator.PointLightError` _returnvalue_2) false false)
    (`SceneComponent.SetVisibility` (`/Game/Blueprints/Actors/Interaction/BP_Interaction_Elevator.PointLightSuccess` _returnvalue_2) true false)
    (`/Game/Blueprints/HI_GameInstance.ShowMessageUI` _ashi_game_instance "Return to Elevator")
    (else
      (`/Game/Blueprints/HI_GameInstance.ShowMessageUI` _ashi_game_instance "Find Remaining Fuses"))))

(fn `UserConstructionScript`
  (`parent.UserConstructionScript`))