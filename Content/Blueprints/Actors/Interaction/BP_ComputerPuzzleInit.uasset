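; BP_ComputerPuzzleInit is an interactable that starts the computer puzzle view once the game instance records that the player has a keyboard.
; On Interact, it finds BP_BlendTriggerVolume and, if unfocused, has it move to BP_CameraComputer.
; After the blend time, it hides the character and shows keyboard actors by tag through HI_GameInstance.
; Without a keyboard, it only prints a hint to find one.
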(event `/Game/Blueprints/Interfaces/BPI_Interaction.Interact`
  (bind _ashi_game_instance (cast `/Game/Blueprints/HI_GameInstance` (`GameplayStatics.GetGameInstance`)))
  (if (`/Game/Blueprints/HI_GameInstance.hasKeyboard` _ashi_game_instance)
    (bind _returnvalue (`GameplayStatics.GetActorOfClass` "/Game/Blueprints/Cameras/BP_BlendTriggerVolume.BP_BlendTriggerVolume_C"))
    (if (not (`/Game/Blueprints/Cameras/BP_BlendTriggerVolume.isFocused` _returnvalue))
      (bind _returnvalue_2 (`GameplayStatics.GetActorOfClass` "/Game/Blueprints/Cameras/BP_CameraComputer.BP_CameraComputer_C"))
      (`/Game/Blueprints/Cameras/BP_BlendTriggerVolume.MoveToCamera` _returnvalue _returnvalue_2)
      (`KismetSystemLibrary.Delay` (`/Game/Blueprints/Cameras/BP_BlendTriggerVolume.CameraBlendTime` _returnvalue))
      (`/Game/Blueprints/Cameras/BP_BlendTriggerVolume.HideCharacter` _returnvalue)
      (`/Game/Blueprints/HI_GameInstance.ShowActorsByTag` _ashi_game_instance "keyboardForComputer")
      (`/Game/Blueprints/HI_GameInstance.ShowActorsByTag` _ashi_game_instance "keyboardForComputerAfterSpawn"))
    (else
      (`KismetSystemLibrary.PrintString` "Find a keyboard"))))

(fn `UserConstructionScript`)