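; Base interactable actor that highlights itself and shows an interaction prompt when the player character is near.
; OutlineCollision overlaps track IsOverlapping and, per option flags, toggle custom depth stencil on the Cube mesh and the player's InteractWidget visibility.
; When CanInteract is off, BeginPlay destroys the collision, disabling both cues.
; Interact is an empty event, and RemoveOutline clears the highlight on demand.
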(event `self.ReceiveBeginPlay`
  (bind _asbp_hiplayer_char (cast `/Game/Blueprints/Characters/PC/BP_HIPlayerChar` (`GameplayStatics.GetPlayerCharacter` 0)))
  (set `self.PlayerRef` null)
  (if (`self.canInteract`)
    (set `self.InteractWidget` (`/Game/Blueprints/Characters/PC/BP_HIPlayerChar.InteractWidget` _asbp_hiplayer_char))
    (else
      (`ActorComponent.K2_DestroyComponent` (`self.OutlineCollision`)))))

(event `/Game/Blueprints/Interfaces/BPI_Interaction.Interact`)

(event `self.OutlineCollision.OnComponentBeginOverlap`
  (params (OverlappedComponent :type "PrimitiveComponent Object Reference") (OtherActor :type "Actor Object Reference") (OtherComp :type "PrimitiveComponent Object Reference") (OtherBodyIndex :type Integer) (bFromSweep :type Boolean) (SweepResult :type "HitResult Structure (by ref)"))
  (bind _cube (`self.Cube`))
  (bind _asbp_hiplayer_char (cast `/Game/Blueprints/Characters/PC/BP_HIPlayerChar` OtherActor))
  (set `self.isOverlapping` true)
  (if (`self.ShowOutline`)
    (`PrimitiveComponent.SetRenderCustomDepth` _cube true)
    (`PrimitiveComponent.SetCustomDepthStencilValue` _cube 1))
  (if (`self.ShowInteractOption`)
    (`Widget.SetVisibility` (`/Game/Blueprints/Characters/PC/BP_HIPlayerChar.InteractWidget` _asbp_hiplayer_char) "Visible")))

(event `self.OutlineCollision.OnComponentEndOverlap`
  (params (OverlappedComponent :type "PrimitiveComponent Object Reference") (OtherActor :type "Actor Object Reference") (OtherComp :type "PrimitiveComponent Object Reference") (OtherBodyIndex :type Integer))
  (bind _asbp_hiplayer_char (cast `/Game/Blueprints/Characters/PC/BP_HIPlayerChar` OtherActor))
  (set `self.isOverlapping` false)
  (if (`self.ShowOutline`)
    (`PrimitiveComponent.SetRenderCustomDepth` (`self.Cube`) false))
  (if (`self.ShowInteractOption`)
    (`Widget.SetVisibility` (`/Game/Blueprints/Characters/PC/BP_HIPlayerChar.InteractWidget` _asbp_hiplayer_char) "Hidden")))

(event `RemoveOutline`
  (`PrimitiveComponent.SetRenderCustomDepth` (`self.Cube`) false))

(fn `UserConstructionScript`)