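; Puzzle interaction actor meant to toggle the player between normal play and a focused puzzle camera.
; ToggleCamera either clears IsFocused and returns the player, or calls MoveCharacterToPuzzle, whose view-target call has no target wired; its focus logic is disconnected.
; ReturnCharacterToGame blends back to the character, restoring HUD, movement and look input and disabling the cursor.
; Tick also calls that return every frame, acting whenever IsFocused is false; Interact only prints debug text.
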(event `/Game/Blueprints/Interfaces/BPI_Interaction.Interact`
  (`KismetSystemLibrary.PrintString` "Not what you expected"))

(event `ToggleCamera`
  ;[0.2154 0.4786 1] Comment
  (`KismetSystemLibrary.PrintString` "If you see this, it's not as pointless as I thought")
  (if (`self.isFocused`)
    (`KismetSystemLibrary.PrintString` "focused")
    (set `self.isFocused` false)
    ;[1 1 1] Comment
    (`self.ReturnCharacterToGame` :!label _label)
    (else
      (`self.Move Character to Puzzle`))))

(event `self.ReceiveTick`
  (params (DeltaSeconds :type "Float (single-precision)"))
  ;[1 1 1] Comment
  (goto _label))

(fn `Move Character to Puzzle`
  (bind _returnvalue (`GameplayStatics.GetActorOfClass` "/Game/Blueprints/Actors/Interaction/Puzzles/BP_PuzzleCircuitBoard.BP_PuzzleCircuitBoard_C"))
  (`PlayerController.SetViewTargetWithBlend` (`GameplayStatics.GetPlayerController` 0) null 0.0 "VTBlend_Linear" 0.0 false))

(fn `ReturnCharacterToGame`
  (bind _returnvalue (`GameplayStatics.GetPlayerController` 0))
  (bind _returnvalue_2 (`GameplayStatics.GetPlayerCharacter` 0))
  ;[1 1 1] Comment
  (if (not (`self.isFocused`))
    (`PlayerController.SetViewTargetWithBlend` _returnvalue _returnvalue_2 (`self.BlendTime`) "VTBlend_Linear" 0.0 false)
    (bind _asl1_character_broken (cast `/Game/Blueprints/Level1/L1_Character` _returnvalue_2))
    (`Widget.SetVisibility` (`/Game/Blueprints/Level1/L1_Character.MainHUDRed` _asl1_character_broken) "Visible")
    (set `PlayerController.bShowMouseCursor` false _returnvalue)
    (set `PlayerController.bEnableClickEvents` false _returnvalue)
    (`ActorComponent.Activate` (`Character.CharacterMovement` _returnvalue_2) false)
    (`Controller.ResetIgnoreLookInput` _returnvalue)))

(fn `UserConstructionScript`
  (`parent.UserConstructionScript`))