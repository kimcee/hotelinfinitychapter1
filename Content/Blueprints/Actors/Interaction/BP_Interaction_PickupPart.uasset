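; BP_Interaction_PickupPart is an interactable part actor that displays its part name on a text render and can be picked up.
; On Interact, a name matching the elevator part sets the Game Instance's elevator-part flag, swaps tagged success and pending actors, and prints guidance.
; Any part, matching or not, clears the waiting-for-pickup flag and shifts its cube along local Y.
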(event `self.ReceiveBeginPlay`
  (`TextRenderComponent.K2_SetText` (`self.TextRender`) (`KismetTextLibrary.Conv_StringToText` (`self.PartName`))))

(event `/Game/Blueprints/Interfaces/BPI_Interaction.Interact`
  (bind _ashi_game_instance (cast `/Game/Blueprints/HI_GameInstance` (`GameplayStatics.GetGameInstance`)))
  (if (`KismetStringLibrary.EqualEqual_StrStr` (`self.PartName`) (`self.ElevatorPartName`))
    (set `/Game/Blueprints/HI_GameInstance.hasElevatorPart` true _ashi_game_instance)
    (`/Game/Blueprints/HI_GameInstance.ShowActorsByTag` _ashi_game_instance "partSuccess")
    (`/Game/Blueprints/HI_GameInstance.HideActorsByTag` _ashi_game_instance "partPending" false)
    (`KismetSystemLibrary.PrintString` "You found the elevator part")
    (`KismetSystemLibrary.PrintString` "Return to elevator gears and add new part"))
  (set `/Game/Blueprints/HI_GameInstance.partGeneratedAndWaitingForPickup` false _ashi_game_instance)
  (`SceneComponent.K2_SetRelativeLocation` (`self.Cube`) (`KismetMathLibrary.MakeVector` 0.0 (`self.New Location Y`)) false false))

(fn `UserConstructionScript`
  (`parent.UserConstructionScript`))