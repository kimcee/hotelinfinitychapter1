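; Interaction button that solves the security lasers puzzle when the player has a keyboard.
; On interact it checks the keyboard flag in HI_GameInstance, then marks the lasers solved and switches the error light to the success light.
; The game instance then destroys obstacle actors by tag and shows tagged items.
; A printed hint points to the level 4 tram station, or to finding a keyboard if none is held.
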(event `/Game/Blueprints/Interfaces/BPI_Interaction.Interact`
  (bind _ashi_game_instance (cast `/Game/Blueprints/HI_GameInstance` (`GameplayStatics.GetGameInstance`)))
  (if (`/Game/Blueprints/HI_GameInstance.hasKeyboard` _ashi_game_instance)
    (set `/Game/Blueprints/HI_GameInstance.hasSolvedSecurityLasers` true _ashi_game_instance)
    (`SceneComponent.SetVisibility` (`Light.LightComponent` (`self.ErrorLight`)) false false)
    (`SceneComponent.SetVisibility` (`Light.LightComponent` (`self.SuccessLight`)) true false)
    ;[1 1 1] Destroy actors that are physical obstacles
    (`/Game/Blueprints/HI_GameInstance.HideActorsByTag` _ashi_game_instance (`self.HideByTag`) true)
    ;[1 1 1] Show relavent items
    (`/Game/Blueprints/HI_GameInstance.ShowActorsByTag` _ashi_game_instance (`self.ShowByTag`))
    (`KismetSystemLibrary.PrintString` "Go to tram station on level 4")
    (else
      (`KismetSystemLibrary.PrintString` "Find a keyboard"))))

(fn `UserConstructionScript`
  (`parent.UserConstructionScript`))