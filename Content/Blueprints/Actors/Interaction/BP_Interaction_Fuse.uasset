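; BP_Interaction_Fuse is an interactable fuse part that can be picked up or shown being slotted into place.
; On BeginPlay it either hides itself or optionally turns off its light and wires, based on instance flags.
; Interacting, when allowed, registers the part with HI_GameInstance, plays a pickup sound and destroys the actor.
; InsertPart reveals a hidden fuse and uses a timeline to lower its cube, ending with a shutter sound.
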(event `self.ReceiveBeginPlay`
  ;[1 0.6702 0.3533] On Load
  (if (`self.isHidden`)
    (`self.SetActorHiddenInGame` true)
    (elif (not (`self.showLight`))
      (`SceneComponent.SetVisibility` (`self.PointLight`) false false)
      (`SceneComponent.SetVisibility` (`self.Wires`) false false)))
  (`parent.ReceiveBeginPlay`))

(event `/Game/Blueprints/Interfaces/BPI_Interaction.Interact`
  ;[0.07746 0.5491 1] Comment
  (if (`self.canInteract`)
    (bind _ashi_game_instance (cast `/Game/Blueprints/HI_GameInstance` (`GameplayStatics.GetGameInstance`)))
    (`/Game/Blueprints/HI_GameInstance.CollectFusePart` _ashi_game_instance)
    (`GameplayStatics.PlaySound2D` "/Engine/VREditor/Sounds/UI/Object_PickUp.Object_PickUp" 1.0 1.0 0.0 null null)
    (`self.K2_DestroyActor`)))

(event `InsertPart`
  (set `self.isHidden` false)
  (`self.SetActorHiddenInGame` false)
  (bind (_direction _alpha) (`Timeline|MovePartIntoPlace`)
    (:`Update`
      (`SceneComponent.K2_SetRelativeLocation` (`self.Cube`) (`KismetMathLibrary.MakeVector` 0.0 0.0 (`KismetMathLibrary.Lerp` 0.0 -50.0 _alpha)) false false))
    (:`Finished`
      (`GameplayStatics.PlaySound2D` "/Engine/VREditor/Sounds/UI/Camera_Shutter.Camera_Shutter" 1.0 1.0 0.0 null null))))

(fn `UserConstructionScript`
  (`parent.UserConstructionScript`))