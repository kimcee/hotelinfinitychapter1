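; Interactable door actor that swings open when the player interacts with it, despite the SlideUp name.
; Interact destroys the outline collision component, then plays a timeline that lerps the door mesh's relative yaw from closed to partly open.
; BeginPlay and construction defer to the parent class, no closing logic exists, and the 2D sound nodes are left unconnected.
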(event `self.ReceiveBeginPlay`
  (`parent.ReceiveBeginPlay`))

(event `/Game/Blueprints/Interfaces/BPI_Interaction.Interact`
  (`ActorComponent.K2_DestroyComponent` (`self.OutlineCollision`))
  (bind (_direction _alpha) (`Timeline|OpenDoorTL`)
    (:`Update`
      (`SceneComponent.K2_SetRelativeRotation` (`self.SM_ChamberXDoor`) (`KismetMathLibrary.MakeRotator` 0.0 0.0 (`KismetMathLibrary.Lerp` 0.0 50.0 _alpha)) false false))))

(fn `UserConstructionScript`
  (`parent.UserConstructionScript`))