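; Interactable card reader that unlocks the main check-in doors once the game instance holds the door key, otherwise prompting to find it.
; On success, it moves the camera to the door view, hides the character and animates the card sliding via timeline.
; It then shows access-granted indicators, disables interaction and opens tagged BP_DoorLockedByID doors.
; Finally, it completes the task, restores the character camera and directs the player to the elevator.
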(event `/Game/Blueprints/Interfaces/BPI_Interaction.Interact`
  ;[0.335 1 0.41] Interact
  (bind _ashi_game_instance (cast `/Game/Blueprints/HI_GameInstance` (`GameplayStatics.GetGameInstance`)))
  (if (`/Game/Blueprints/HI_GameInstance.hasDoorKey` _ashi_game_instance)
    (set `/Game/Blueprints/HI_GameInstance.hasUnlockedMainDoors` true _ashi_game_instance)
    (`self.PlayAnimation`)
    (else
      (`/Game/Blueprints/HI_GameInstance.ShowMessageUI` _ashi_game_instance "Find Door Key"))))

(event `PlayAnimation`
  ;[0 0 0] Solved
  ;[0.9206 0.2355 1] Focus Character Camera
  (bind _returnvalue (`GameplayStatics.GetActorOfClass` "/Game/Blueprints/Cameras/BP_BlendTriggerVolume.BP_BlendTriggerVolume_C"))
  (if (not (`/Game/Blueprints/Cameras/BP_BlendTriggerVolume.isFocused` _returnvalue))
    (bind _returnvalue_2 (`GameplayStatics.GetActorOfClass` "/Game/Blueprints/Cameras/BP_CameraDoor.BP_CameraDoor_C"))
    (`/Game/Blueprints/Cameras/BP_BlendTriggerVolume.MoveToCamera` _returnvalue _returnvalue_2)
    (`KismetSystemLibrary.Delay` 0.8)
    (`/Game/Blueprints/Cameras/BP_BlendTriggerVolume.HideCharacter` _returnvalue)
    ;[1 0.3024 0.2962] AnimateDoorOpening
    (`SceneComponent.SetVisibility` (`self.DoorCard`) true false)
    (bind (_direction _alpha) (`Timeline|SlideCardTL` :!via `PlayFromStart`)
      (:`Update`
        (`SceneComponent.K2_SetRelativeLocation` (`self.DoorCard`) (`KismetMathLibrary.MakeVector` (`KismetMathLibrary.Lerp` 25.0 -135.0 _alpha) (`KismetMathLibrary.Lerp` 42.0 -240.0 _alpha) (`KismetMathLibrary.Lerp` 5.0 2.0 _alpha)) false false))
      (:`Finished`
        (`PrimitiveComponent.SetMaterial` (`self.CardReaderStatus`) 0 "/Engine/MapTemplates/Materials/BasicAsset03.BasicAsset03")
        (`self.MakeAccessGranted`)
        (set `self.canInteract` false)
        (set `self.ShowInteractOption` false)
        (set `self.ShowOutline` false)
        (`self.RemoveOutline`)
        (bind _outactors (`GameplayStatics.GetAllActorsOfClassWithTag` "/Game/Blueprints/Actors/Interaction/BP_DoorLockedByID.BP_DoorLockedByID_C" "CheckinDoor"))
        (for _array_element _outactors
          (`/Game/Blueprints/Actors/Interaction/BP_DoorLockedByID.OpenDoor` _array_element))
        ;[1 1 1] Comment
        (bind _ashi_game_instance (cast `/Game/Blueprints/HI_GameInstance` (`GameplayStatics.GetGameInstance`)))
        (`/Game/Blueprints/HI_GameInstance.TaskComplete` _ashi_game_instance)
        (set `/Game/Blueprints/HI_GameInstance.hasUnlockedMainDoors` true _ashi_game_instance)
        (bind _returnvalue_3 (`GameplayStatics.GetActorOfClass` "/Game/Blueprints/Cameras/BP_BlendTriggerVolume.BP_BlendTriggerVolume_C"))
        (`/Game/Blueprints/Cameras/BP_BlendTriggerVolume.ReturnToCharacter` _returnvalue_3)
        (`/Game/Blueprints/HI_GameInstance.ShowMessageUI` _ashi_game_instance "Go to the Elevator")))))

(fn `MakeAccessDenied`
  (bind _outactors (`GameplayStatics.GetAllActorsWithTag` "doorAccessDenied"))
  (for _array_element _outactors
    (`SceneComponent.SetVisibility` (`Actor.RootComponent` _array_element) true false))
  (bind _outactors_2 (`GameplayStatics.GetAllActorsWithTag` "doorAccessGranted"))
  (for _array_element_2 _outactors_2
    (`SceneComponent.SetVisibility` (`Actor.RootComponent` _array_element_2) false false))
  (`KismetSystemLibrary.PrintString` "You must use your key again"))

(fn `MakeAccessGranted`
  (bind _outactors (`GameplayStatics.GetAllActorsWithTag` "doorAccessGranted"))
  (for _array_element _outactors
    (`SceneComponent.SetVisibility` (`Actor.RootComponent` _array_element) true false))
  (bind _outactors_2 (`GameplayStatics.GetAllActorsWithTag` "doorAccessDenied"))
  (for _array_element_2 _outactors_2
    (`SceneComponent.SetVisibility` (`Actor.RootComponent` _array_element_2) false false))
  (`KismetSystemLibrary.PrintString` "You may now enter the doors")
  (`GameplayStatics.PlaySound2D` "/Engine/VREditor/Sounds/UI/Enter_Play.Enter_Play" 1.0 1.0 0.0 null null))

(fn `UserConstructionScript`
  (`parent.UserConstructionScript`))