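; Interactable button that generates either a door or tram key card, once the game instance flags the generator as unlocked and no key is already generated.
; Interact sets the generated flag, swaps to pressed visuals, and compares CardType to DefaultCardType as text to choose which pickup class's actors reveal their card.
; It also switches the other card option from access-granted to access-required by hiding and showing tagged actors through the game instance.
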(event `/Game/Blueprints/Interfaces/BPI_Interaction.Interact`
  (bind _ashi_game_instance (cast `/Game/Blueprints/HI_GameInstance` (`GameplayStatics.GetGameInstance`)))
  (if (`/Game/Blueprints/HI_GameInstance.hasGeneratedKey` _ashi_game_instance)
    (`KismetSystemLibrary.PrintString` "Key has already been generated, pickup key to re-allow")
    (elif (`/Game/Blueprints/HI_GameInstance.hasUnlockedKeyGenerator` _ashi_game_instance)
      (set `/Game/Blueprints/HI_GameInstance.hasGeneratedKey` true _ashi_game_instance)
      (`self.setPressed`)
      (if (`KismetTextLibrary.EqualEqual_TextText` (`KismetTextLibrary.Conv_StringToText` (`self.CardType`)) (`KismetTextLibrary.Conv_StringToText` (`self.DefaultCardType`)))
        ;[1 1 1] Show Door Key Card
        (bind _outactors (`GameplayStatics.GetAllActorsOfClass` "/Game/Blueprints/Actors/Interaction/BP_Interaction_ButtonPickupKey1.BP_Interaction_ButtonPickupKey1_C"))
        (for _array_element _outactors
          (`/Game/Blueprints/Actors/Interaction/BP_Interaction_ButtonPickupKey1.showCard` _array_element))
        ;[1 1 1] Hide Tram Card Option
        (`/Game/Blueprints/HI_GameInstance.HideActorsByTag` _ashi_game_instance "tramCardAccessGranted" false)
        (`/Game/Blueprints/HI_GameInstance.ShowActorsByTag` _ashi_game_instance "tramCardAccessRequired")
        (else
          ;[1 1 1] Show Tram Key Card
          (bind _outactors_2 (`GameplayStatics.GetAllActorsOfClass` "/Game/Blueprints/Actors/Interaction/BP_Interaction_ButtonPickupKey2.BP_Interaction_ButtonPickupKey2_C"))
          (for _array_element_2 _outactors_2
            (`/Game/Blueprints/Actors/Interaction/BP_Interaction_ButtonPickupKey2.showCard` _array_element_2))
          ;[1 1 1] Hide Door Card Option
          (`/Game/Blueprints/HI_GameInstance.HideActorsByTag` _ashi_game_instance "doorCardAccessGranted" false)
          (`/Game/Blueprints/HI_GameInstance.ShowActorsByTag` _ashi_game_instance "doorCardAccessRequired")))
      (else
        (`KismetSystemLibrary.PrintString` "access denied")))))

(fn `setPressed`
  (`SceneComponent.SetVisibility` (`self.Cube`) false false)
  (`SceneComponent.SetVisibility` (`self.CubePress`) true false)
  (`SceneComponent.SetVisibility` (`self.PointLightPress`) true false))

(fn `setUnPressed`
  (`SceneComponent.SetVisibility` (`self.Cube`) true false)
  (`SceneComponent.SetVisibility` (`self.CubePress`) false false)
  (`SceneComponent.SetVisibility` (`self.PointLightPress`) false false))

(fn `UserConstructionScript`
  (`parent.UserConstructionScript`))