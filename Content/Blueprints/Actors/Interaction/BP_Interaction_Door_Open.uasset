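; Interactable electrical panel door that opens only when the game instance reports the player has the prying tool, otherwise showing a hint.
; Interact swings the door via timeline, plays a shutter sound, clears hints and outline, and focuses the BP_BlendTriggerVolume camera, hiding the character.
; Interacting while open only refocuses the camera.
; CloseDoor reverses the swing and disables interaction; BeginPlay removes outline collision if already solved.
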(event `self.ReceiveBeginPlay`
  ;[1 0.2234 0.04558] EventBegin
  (bind _ashi_game_instance (cast `/Game/Blueprints/HI_GameInstance` (`GameplayStatics.GetGameInstance`)))
  (bind _hassolved (`/Game/Blueprints/HI_GameInstance.GetHasSolved` _ashi_game_instance (`self.HasSolvedVariable`)))
  (if _hassolved
    (`ActorComponent.K2_DestroyComponent` (`self.OutlineCollision`))))

(event `/Game/Blueprints/Interfaces/BPI_Interaction.Interact`
  ;[0.2154 0.4786 1] Comment
  (bind _ashi_game_instance (cast `/Game/Blueprints/HI_GameInstance` (`GameplayStatics.GetGameInstance`)))
  (if (`/Game/Blueprints/HI_GameInstance.hasPryingTool` _ashi_game_instance)
    (if (`self.isDoorClosed`)
      (set `self.isDoorClosed` false)
      (`|ExecutionSequence`
        (:`then_0`
          (bind (_direction _newtrack_0) (`Timeline|OpenDoorTL` :!via `PlayFromStart` :!label _label)
            (:`Update`
              (`SceneComponent.K2_SetRelativeRotation` (`self.Cube`) (`KismetMathLibrary.MakeRotator` (`KismetMathLibrary.Lerp` 0.0 90.0 _newtrack_0)) false false))))
        (:`then_1`
          ;[0.9206 0.2355 1] Focus Character Camera
          (bind _returnvalue (`GameplayStatics.GetActorOfClass` "/Game/Blueprints/Cameras/BP_BlendTriggerVolume.BP_BlendTriggerVolume_C" :!label _label_2))
          (if (not (`/Game/Blueprints/Cameras/BP_BlendTriggerVolume.isFocused` _returnvalue))
            (`/Game/Blueprints/Cameras/BP_BlendTriggerVolume.MoveToCamera` _returnvalue (`self.CameraToFocus`))
            (`KismetSystemLibrary.Delay` 0.8)
            (`/Game/Blueprints/Cameras/BP_BlendTriggerVolume.HideCharacter` _returnvalue)))
        (:`then_2`
          (`GameplayStatics.PlaySound2D` "/Engine/VREditor/Sounds/UI/Camera_Shutter.Camera_Shutter" 1.0 1.0 0.0 null null false :!label _label_3))
        (:`then_3`
          ;[0.203 0.7728 1] Comment
          (bind _asbp_hiplayer_char (cast `/Game/Blueprints/Characters/PC/BP_HIPlayerChar` (`GameplayStatics.GetPlayerCharacter` 0)))
          (`/Game/UI/WBP_UserHints.ClearMessage` (`/Game/Blueprints/Characters/PC/BP_HIPlayerChar.UserHintsWidget` _asbp_hiplayer_char)))
        (:`then_4`
          (set `self.ShowOutline` false)
          (`self.RemoveOutline`)))
      (else
        (goto _label_2)))
    (else
      ;[1 0.8929 0.2071] Comment
      (`/Game/Blueprints/HI_GameInstance.ShowMessageUI` _ashi_game_instance "Find prying tool to open electrical panel"))))

(event `CloseDoor`
  ;[0.3759 1 0.9198] Close Door
  (`|ExecutionSequence`
    (:`then_0`
      (goto _label :!via `ReverseFromEnd`))
    (:`then_1`
      (goto _label_3))
    (:`then_2`
      (set `self.canInteract` false))
    (:`then_3`
      (set `self.ShowInteractOption` false))))

(fn `UserConstructionScript`
  (`parent.UserConstructionScript`))