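; Countdown timer actor for a laser lockdown sequence, with an on-screen widget and music.
; BeginTimer resets the time, shows the widget, starts music, moves all lasers into place and starts RunTimer, which re-calls itself after one-second delays.
; At zero it stops camera shake, hides the widget and deactivates music.
; If KillPlayer is set, it then waits the player's death pause and resets all lockdown pillars and lasers.
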(event `RunTimer`
  ;[1 0.3086 0.7653] Initiate Timer
  (if (`self.isTimerActive`)
    (`KismetSystemLibrary.Delay` 1.0)
    (if (== (`self.Seconds`) 0)
      (if (== (`self.Minutes`) 0)
        (set `self.isTimerActive` false)
        (`self.StopTimer`)
        (if (`self.killPlayer`)
          (`self.KillPlayerDuringTimerRun`))
        (else
          (set `self.Seconds` 59)
          (set `self.Minutes` (- (`self.Minutes`) 1))
          (`self.RunTimer` :!label _label)))
      (else
        (set `self.Seconds` (- (`self.Seconds`) 1))
        (goto _label)))))

(event `StopTimer`
  ;[0.3253 1 0.8009] Stop Timer
  (set `self.isTimerActive` false)
  (bind _asbp_hiplayer_char (cast `/Game/Blueprints/Characters/PC/BP_HIPlayerChar` (`GameplayStatics.GetPlayerCharacter` 0)))
  (`/Game/Blueprints/Characters/PC/BP_HIPlayerChar.StopCameraShake` _asbp_hiplayer_char)
  (`Widget.SetVisibility` (`self.TimerWidget`) "Hidden")
  (`ActorComponent.SetActive` (`self.Music`) false false))

(event `BeginTimer`
  ;[0.2678 0.218 1] Begin The Timer Counter
  (`self.CreateWidget`)
  (`self.SetTimer`)
  (set `self.isTimerActive` true)
  (bind _returnvalue (`GameplayStatics.SpawnSound2D` null 0.5 1.0 2.0 null))
  (bind _output_get (set `self.Music` _returnvalue))
  (`ActorComponent.SetActive` _output_get true false)
  (`self.RunTimer`)
  ;[1 0 0.01045] Move Lazers into Place
  (bind _outactors (`GameplayStatics.GetAllActorsOfClass` "/Game/Blueprints/Actors/AIActors/BP_LazerMoveIntoPlace.BP_LazerMoveIntoPlace_C"))
  (for _array_element _outactors
    (`/Game/Blueprints/Actors/AIActors/BP_LazerMoveIntoPlace.MoveIntoPlace` _array_element)))

(event `SetTimer`
  ;[1 0.1877 0.2295] Set The Timer
  (set `self.Minutes` (`self.MinutesDefault`))
  (set `self.Seconds` (`self.SecondsDefault`)))

(event `StopTimerMusic`
  ;[1 1 1] Stop Music
  (`AudioComponent.Stop` (`self.Music`)))

(event `KillPlayerDuringTimerRun`
  ;[0 0 0] Kill Player and Reset Everything
  (`self.StopTimer`)
  (bind _asbp_hiplayer_char (cast `/Game/Blueprints/Characters/PC/BP_HIPlayerChar` (`GameplayStatics.GetPlayerCharacter` 0)))
  (`KismetSystemLibrary.Delay` (`/Game/Blueprints/Characters/PC/BP_HIPlayerChar.PlayerDiedPause` _asbp_hiplayer_char))
  (bind _outactors (`GameplayStatics.GetAllActorsOfClass` "/Game/Blueprints/Actors/Movement/BP_LockdownPillars.BP_LockdownPillars_C"))
  (for _array_element _outactors
    (`/Game/Blueprints/Actors/Movement/BP_LockdownPillars.ResetPillar` _array_element))
  (bind _outactors_2 (`GameplayStatics.GetAllActorsOfClass` "/Game/Blueprints/Actors/AIActors/BP_LazerMoveIntoPlace.BP_LazerMoveIntoPlace_C"))
  (for _array_element_2 _outactors_2
    (`/Game/Blueprints/Actors/AIActors/BP_LazerMoveIntoPlace.ResetLazer` _array_element_2)))

(fn `CreateWidget`
  (bind _returnvalue (`|CreateWidget` "/Game/UI/WBP_Timer.WBP_Timer_C"))
  (bind _output_get (set `self.TimerWidget` _returnvalue))
  (`UserWidget.AddToViewport` _output_get 0)
  (`Widget.SetVisibility` _output_get "Visible"))

(fn `UserConstructionScript`
  (`parent.UserConstructionScript`))