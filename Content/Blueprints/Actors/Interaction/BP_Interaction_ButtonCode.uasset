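; BP_Interaction_ButtonCode is a numbered keypad button for the access card generator code puzzle, displaying its value on a text label.
; A click presses it once, changing mesh position and material, then sends its value to the BP_AccessCardGenerator found in the level.
; A true return plays a failure sound and flashes then resets the buttons; otherwise, the GameInstance unlock flag triggers the authorization message.
; Interact is empty, leaving MoveCharacterToPuzzle unused.
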(event `self.ReceiveBeginPlay`
  ;[1 1 1] Begin
  (`TextRenderComponent.K2_SetText` (`self.ButtonNumber`) (`KismetTextLibrary.Conv_StringToText` (`self.ButtonValue`)))
  (`parent.ReceiveBeginPlay`))

(event `/Game/Blueprints/Interfaces/BPI_Interaction.MouseClick`
  ;[1 1 1] Interact with Button
  (if (not (`self.isPressed`))
    (`self.PressButton`)
    (bind _returnvalue (`GameplayStatics.GetActorOfClass` "/Game/Blueprints/Actors/Interaction/BP_AccessCardGenerator.BP_AccessCardGenerator_C"))
    (bind _resetcode (`/Game/Blueprints/Actors/Interaction/BP_AccessCardGenerator.UpdateCodeEntered` _returnvalue (`self.ButtonValue`)))
    (if _resetcode
      (`GameplayStatics.PlaySound2D` "/Engine/EditorSounds/Notifications/CompileFailed.CompileFailed" 1.0 1.0 0.0 null null)
      (`/Game/Blueprints/Actors/Interaction/BP_AccessCardGenerator.ErrorButtons` _returnvalue)
      (`KismetSystemLibrary.Delay` 0.2)
      (`/Game/Blueprints/Actors/Interaction/BP_AccessCardGenerator.ResetButtons` _returnvalue)
      (else
        (bind _ashi_game_instance (cast `/Game/Blueprints/HI_GameInstance` (`GameplayStatics.GetGameInstance`)))
        (if (`/Game/Blueprints/HI_GameInstance.hasUnlockedKeyGenerator` _ashi_game_instance)
          (`GameplayStatics.PlaySound2D` "/Engine/EditorSounds/Notifications/CompileSuccess.CompileSuccess" 1.0 1.0 0.0 null null)
          (`/Game/Blueprints/HI_GameInstance.ShowMessageUI` _ashi_game_instance "Key Access Authorized"))))))

(event `PressButton`
  (bind _cube (`self.Cube`))
  ;[1 1 1] Button Press Action
  (`SceneComponent.K2_SetRelativeLocation` _cube (0.0 0.0 -2.0) false false)
  (set `self.isPressed` true)
  (`PrimitiveComponent.SetMaterial` _cube 0 "/Engine/MapTemplates/Materials/BasicAsset03.BasicAsset03")
  (`GameplayStatics.PlaySound2D` "/Game/Audio/beep_03.beep_03" 1.0 1.0 0.0 null null))

(event `ResetButton`
  (bind _cube (`self.Cube`))
  ;[1 1 1] Button Press Action
  (`SceneComponent.K2_SetRelativeLocation` _cube (0.0 0.0 0.0) false false)
  (set `self.isPressed` false)
  (`PrimitiveComponent.SetMaterial` _cube 0 "/Engine/BasicShapes/BasicShapeMaterial.BasicShapeMaterial")
  (`GameplayStatics.PlaySound2D` null 1.0 1.0 0.0 null null))

(event `ErrorButton`
  ;[1 1 1] Button Press Action
  (`PrimitiveComponent.SetMaterial` (`self.Cube`) 0 "/Engine/MapTemplates/Materials/BasicAsset01.BasicAsset01"))

(event `/Game/Blueprints/Interfaces/BPI_Interaction.Interact`
  ;[0.9206 0.2355 1] Focus Character Camera
)

(fn `UserConstructionScript`
  (`parent.UserConstructionScript`))