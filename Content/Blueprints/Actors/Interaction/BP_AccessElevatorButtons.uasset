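; BP_AccessElevatorButtons is an interactable actor that grants access to the elevator buttons once the elevator puzzle is solved.
; On Interact it checks the solved flag on HI_GameInstance and shows a "Fix Elevator" message when unsolved.
; When solved and not already focused, it has BP_BlendTriggerVolume move the view to BP_CameraElevator, then hides the character after a short delay.
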(event `/Game/Blueprints/Interfaces/BPI_Interaction.Interact`
  (bind _ashi_game_instance (cast `/Game/Blueprints/HI_GameInstance` (`GameplayStatics.GetGameInstance`)))
  (if (`/Game/Blueprints/HI_GameInstance.hasSolvedElevatorPuzzle` _ashi_game_instance)
    (bind _returnvalue (`GameplayStatics.GetActorOfClass` "/Game/Blueprints/Cameras/BP_BlendTriggerVolume.BP_BlendTriggerVolume_C"))
    (if (not (`/Game/Blueprints/Cameras/BP_BlendTriggerVolume.isFocused` _returnvalue))
      (bind _returnvalue_2 (`GameplayStatics.GetActorOfClass` "/Game/Blueprints/Cameras/BP_CameraElevator.BP_CameraElevator_C"))
      (`/Game/Blueprints/Cameras/BP_BlendTriggerVolume.MoveToCamera` _returnvalue _returnvalue_2)
      (`KismetSystemLibrary.Delay` 0.8)
      (`/Game/Blueprints/Cameras/BP_BlendTriggerVolume.HideCharacter` _returnvalue))
    (else
      (`/Game/Blueprints/HI_GameInstance.ShowMessageUI` _ashi_game_instance "Fix Elevator"))))

(fn `UserConstructionScript`)