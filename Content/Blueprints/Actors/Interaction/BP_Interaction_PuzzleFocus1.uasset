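; Puzzle-focus interaction actor, apparently an unfinished or debug version of a camera toggle between the player character and a puzzle.
; ToggleCamera flips IsFocused with debug prints, while Interact only prints a message.
; Tick calls ReturnCharacterToGame every frame, but that function is empty.
; Logic for view blending, HUD visibility, cursor and movement locking sits disconnected in both focus functions, so it never runs.
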(event `/Game/Blueprints/Interfaces/BPI_Interaction.Interact`
  (`KismetSystemLibrary.PrintString` "Not what you expected"))

(event `ToggleCamera`
  ;[0.2154 0.4786 1] Comment
  (`KismetSystemLibrary.PrintString` "If you see this, it's not as pointless as I thought")
  (if (`self.isFocused`)
    (`KismetSystemLibrary.PrintString` "focused")
    (set `self.isFocused` false)
    ;[1 1 1] Comment
    (`self.ReturnCharacterToGame` :!label _label)
    (else
      (`self.MoveCharacterToPuzzle`))))

(event `self.ReceiveTick`
  (params (DeltaSeconds :type "Float (single-precision)"))
  ;[1 1 1] Comment
  (goto _label))

(fn `MoveCharacterToPuzzle`
  (`KismetSystemLibrary.PrintString` "Trying to focus")
  ;[1 1 1] Character Movement
  (set `self.isFocused` true))

(fn `ReturnCharacterToGame`
  ;[1 1 1] Comment
)

(fn `UserConstructionScript`
  (`parent.UserConstructionScript`))