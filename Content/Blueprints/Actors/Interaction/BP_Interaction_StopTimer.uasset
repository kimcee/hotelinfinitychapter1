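; Interaction actor that stops the level's kill timer once the spark plug puzzle is solved.
; An overlap on its OutlineCollision by the L1_Character, gated by the IsPressed flag, checks the solved state in HI_GameInstance.
; On success it finds the BP_Timer by class, clears its KillPlayer flag and destroys itself.
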(event `self.OutlineCollision.OnComponentBeginOverlap`
  (params (OverlappedComponent :type "PrimitiveComponent Object Reference") (OtherActor :type "Actor Object Reference") (OtherComp :type "PrimitiveComponent Object Reference") (OtherBodyIndex :type Integer) (bFromSweep :type Boolean) (SweepResult :type "HitResult Structure (by ref)"))
  (if (`self.isPressed`)
    (cast `/Game/Blueprints/Level1/L1_Character` OtherActor)
    (bind _ashi_game_instance (cast `/Game/Blueprints/HI_GameInstance` (`GameplayStatics.GetGameInstance`)))
    (`KismetSystemLibrary.PrintString` "Try to stop timer")
    (if (`/Game/Blueprints/HI_GameInstance.hasSolvedSparkPlugPuzzle` _ashi_game_instance)
      (set `self.isPressed` true)
      (bind _returnvalue (`GameplayStatics.GetActorOfClass` "/Game/Blueprints/Level1/BP_Timer.BP_Timer_C"))
      (set `/Game/Blueprints/Level1/BP_Timer.killPlayer` false _returnvalue)
      (`self.K2_DestroyActor`))))

(fn `UserConstructionScript`
  (`parent.UserConstructionScript`))