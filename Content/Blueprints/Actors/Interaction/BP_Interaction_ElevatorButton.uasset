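; Clickable elevator floor button interaction actor that sends the elevator to its assigned floor.
; A mouse click works only once the game instance reports the elevator puzzle solved.
; It returns the camera to the character through the blend trigger volume, waits briefly, then sets the destination floor on every elevator actor in the level and starts it moving.
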(event `self.ReceiveBeginPlay`
  (`parent.ReceiveBeginPlay`))

(event `/Game/Blueprints/Interfaces/BPI_Interaction.MouseClick`
  (bind _ashi_game_instance (cast `/Game/Blueprints/HI_GameInstance` (`GameplayStatics.GetGameInstance`)))
  (if (`/Game/Blueprints/HI_GameInstance.hasSolvedElevatorPuzzle` _ashi_game_instance)
    (bind _returnvalue (`GameplayStatics.GetActorOfClass` "/Game/Blueprints/Cameras/BP_BlendTriggerVolume.BP_BlendTriggerVolume_C"))
    (`/Game/Blueprints/Cameras/BP_BlendTriggerVolume.ReturnToCharacter` _returnvalue)
    (`KismetSystemLibrary.Delay` 0.1)
    (bind _outactors (`GameplayStatics.GetAllActorsOfClass` "/Game/Blueprints/Actors/Interaction/BP_Interaction_Elevator.BP_Interaction_Elevator_C"))
    (for _array_element _outactors
      (set `/Game/Blueprints/Actors/Interaction/BP_Interaction_Elevator.DestinationFloor` (`self.ClickedFloor`) _array_element)
      (`/Game/Blueprints/Actors/Interaction/BP_Interaction_Elevator.Move Elevator` _array_element))))

(fn `UserConstructionScript`
  (`parent.UserConstructionScript`))