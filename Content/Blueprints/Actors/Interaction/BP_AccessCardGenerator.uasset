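; Keypad puzzle actor for an access card generator that checks an entered code against the access code.
; UpdateCodeEntered appends button values; at full length, a wrong code clears input and returns true as an error.
; A match completes the game instance task, flags the generator unlocked, swaps tagged access-required/granted visuals and returns the player to character through BP_BlendTriggerVolume.
; Helper functions reset all code buttons, flag pressed ones as errors or restore restricted visuals.
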(fn `ErrorButtons`
  (bind _outactors (`GameplayStatics.GetAllActorsOfClass` "/Game/Blueprints/Actors/Interaction/BP_Interaction_ButtonCode.BP_Interaction_ButtonCode_C"))
  (for _array_element _outactors
    (if (`/Game/Blueprints/Actors/Interaction/BP_Interaction_ButtonCode.isPressed` _array_element)
      (`/Game/Blueprints/Actors/Interaction/BP_Interaction_ButtonCode.ErrorButton` _array_element))))

(fn `ResetButtons`
  (bind _outactors (`GameplayStatics.GetAllActorsOfClass` "/Game/Blueprints/Actors/Interaction/BP_Interaction_ButtonCode.BP_Interaction_ButtonCode_C"))
  (for _array_element _outactors
    (`/Game/Blueprints/Actors/Interaction/BP_Interaction_ButtonCode.ResetButton` _array_element))
  (set `self.CodeEntered` "")
  (set `self.CodeLength` 0))

(fn `showAccessGranted`
  (bind _outactors (`GameplayStatics.GetAllActorsWithTag` "accessRequired"))
  (for _array_element _outactors
    (`SceneComponent.SetVisibility` (`Actor.RootComponent` _array_element) false false))
  (bind _outactors_2 (`GameplayStatics.GetAllActorsWithTag` "accessGranted"))
  (for _array_element_2 _outactors_2
    (`SceneComponent.SetVisibility` (`Actor.RootComponent` _array_element_2) true false)))

(fn `showAccessRestricted`
  (bind _outactors (`GameplayStatics.GetAllActorsWithTag` "accessRequired"))
  (for _array_element _outactors
    (`SceneComponent.SetVisibility` (`Actor.RootComponent` _array_element) true false))
  (bind _outactors_2 (`GameplayStatics.GetAllActorsWithTag` "accessGranted"))
  (for _array_element_2 _outactors_2
    (`SceneComponent.SetVisibility` (`Actor.RootComponent` _array_element_2) false false)))

(fn `UpdateCodeEntered`
  (params (ButtonValue :type String))
  (returns (resetCode :type Boolean))
  (bind _codemaxlength (`self.CodeMaxLength`))
  (bind _output_get (set `self.CodeLength` (+ (`self.CodeLength`) 1)))
  (if (> _output_get _codemaxlength)
    (set `self.CodeEntered` ""))
  (bind _output_get_2 (set `self.CodeEntered` (`KismetStringLibrary.Concat_StrStr` (`self.CodeEntered`) ButtonValue)))
  (if (== _output_get _codemaxlength)
    (if (`KismetStringLibrary.EqualEqual_StrStr` _output_get_2 (`self.AccessCode`))
      (bind _ashi_game_instance (cast `/Game/Blueprints/HI_GameInstance` (`GameplayStatics.GetGameInstance`)))
      (`/Game/Blueprints/HI_GameInstance.TaskComplete` _ashi_game_instance)
      (set `/Game/Blueprints/HI_GameInstance.hasUnlockedKeyGenerator` true _ashi_game_instance)
      (`self.showAccessGranted`)
      ;[1 1 1] Return player to game
      (bind _returnvalue (`GameplayStatics.GetActorOfClass` "/Game/Blueprints/Cameras/BP_BlendTriggerVolume.BP_BlendTriggerVolume_C"))
      (`/Game/Blueprints/Cameras/BP_BlendTriggerVolume.ReturnToCharacter` _returnvalue)
      (return false)
      (else
        (set `self.CodeEntered` "")
        (set `self.CodeLength` 0)
        (`KismetSystemLibrary.PrintString` "Invalid Code, try again")
        (return true)))
    (else
      (return false))))

(fn `UserConstructionScript`)