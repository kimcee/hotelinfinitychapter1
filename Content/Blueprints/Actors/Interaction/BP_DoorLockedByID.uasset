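; BP_DoorLockedByID is a locked double door tied to a solved flag, looked up on HI_GameInstance through HasSolvedVariable.
; On BeginPlay, a solved flag snaps both panels to preset offsets, which differ from the timeline's end positions.
; The OpenDoor event slides the panels apart on a timeline with a sound that stops on finish.
; Player overlap with Collision only shows the locked message while unsolved; it never opens the door.
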(event `self.ReceiveBeginPlay`
  (bind _ashi_game_instance (cast `/Game/Blueprints/HI_GameInstance` (`GameplayStatics.GetGameInstance`)))
  (bind _hassolved (`/Game/Blueprints/HI_GameInstance.GetHasSolved` _ashi_game_instance (`self.HasSolvedVariable`)))
  (if _hassolved
    (`SceneComponent.K2_SetRelativeLocation` (`self.DoorR`) (0.0 155.0 0.0) false false)
    (`SceneComponent.K2_SetRelativeLocation` (`self.DoorL`) (0.0 -155.0 0.0) false false)))

(event `OpenDoor`
  ;[0.07626 0.397 1] Open Door
  (bind _returnvalue (`GameplayStatics.SpawnSound2D` null 1.0 1.0 0.0 null))
  (set `self.DoorOpenSound` _returnvalue)
  (bind (_direction _alpha) (`Timeline|DoorOpenTL` :!via `PlayFromStart`)
    (:`Update`
      (`SceneComponent.K2_SetRelativeLocation` (`self.DoorR`) (`KismetMathLibrary.MakeVector` 0.0 (`KismetMathLibrary.Lerp` -195.0 -300.0 _alpha)) false false)
      (`SceneComponent.K2_SetRelativeLocation` (`self.DoorL`) (`KismetMathLibrary.MakeVector` 0.0 (`KismetMathLibrary.Lerp` 195.0 300.0 _alpha)) false false))
    (:`Finished`
      (`AudioComponent.Stop` (`self.DoorOpenSound`)))))

(event `self.Collision.OnComponentBeginOverlap`
  (params (OverlappedComponent :type "PrimitiveComponent Object Reference") (OtherActor :type "Actor Object Reference") (OtherComp :type "PrimitiveComponent Object Reference") (OtherBodyIndex :type Integer) (bFromSweep :type Boolean) (SweepResult :type "HitResult Structure (by ref)"))
  ;[0.07314 1 0.393] Try to open Door
  (cast `/Game/Blueprints/Characters/PC/BP_HIPlayerChar` OtherActor)
  (bind _ashi_game_instance (cast `/Game/Blueprints/HI_GameInstance` (`GameplayStatics.GetGameInstance`)))
  (bind _hassolved (`/Game/Blueprints/HI_GameInstance.GetHasSolved` _ashi_game_instance (`self.HasSolvedVariable`)))
  (if (not _hassolved)
    (`/Game/Blueprints/HI_GameInstance.ShowMessageUI` _ashi_game_instance (`self.DoorLockedMessage`))))

(fn `UserConstructionScript`)