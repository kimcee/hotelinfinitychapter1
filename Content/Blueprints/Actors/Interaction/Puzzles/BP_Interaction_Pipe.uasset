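; BP_Interaction_Pipe is a rotatable pipe tile for a circuit board puzzle.
; SetupPipe applies the starting angle and hides unused top, right, bottom or left segments.
; A mouse click plays a sound and turns the rotator a quarter turn via a timeline lerp, ignoring clicks while moving.
; It then compares the angle to the correct one within a tolerance, sets IsCorrect and, on a match, asks CircuitBoard to validate the puzzle.
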(event `SetupPipe`
  ;[1 1 1] Begin
  (`SceneComponent.K2_SetRelativeRotation` (`self.RotatorObject`) (`KismetMathLibrary.MakeRotator` 0.0 (`self.CurrentRotationAngle`)) false false)
  (`|ExecutionSequence`
    (:`then_0`
      (if (not (`self.showPipeTop`))
        (`SceneComponent.SetVisibility` (`self.PipeTop`) false false)))
    (:`then_1`
      (if (not (`self.showPipeRight`))
        (`SceneComponent.SetVisibility` (`self.PipeRight`) false false)))
    (:`then_2`
      (if (not (`self.showPipeBottom`))
        (`SceneComponent.SetVisibility` (`self.PipeBottom`) false false)))
    (:`then_3`
      (if (not (`self.showPipeLeft`))
        (`SceneComponent.SetVisibility` (`self.PipeLeft`) false false)))))

(event `self.MouseClick`
  ;[0.1421 0.584 1] Interact Option - can be triggered by mouse click (see l1 character event graph) must have collision type as WorldDynamic
  ;;[1 1 1] Mouse Click Interaction
  (`/Engine/EditorBlueprintResources/StandardMacros.IsValid` (`self.RotatorObject`)
    (:`Is Valid`
      (if (not (`self.isMoving`))
        (set `self.isMoving` true)
        (bind _rotationangle (`self.getNextRotationAngle`))
        (`GameplayStatics.PlaySound2D` null 0.4 1.0 0.0 null null)
        (bind (_direction _newtrack_0) (`Timeline|RotateMesh` :!via `PlayFromStart`)
          (:`Update`
            (`SceneComponent.K2_SetRelativeRotation` (`self.RotatorObject`) (`KismetMathLibrary.MakeRotator` 0.0 (`KismetMathLibrary.Lerp` (`self.CurrentRotationAngle`) _rotationangle _newtrack_0)) false false))
          (:`Finished`
            (set `self.CurrentRotationAngle` _rotationangle)
            (`self.ValidateAngle`)
            (set `self.isMoving` false)))))))

(event `self.Interact`)

(event `ValidateAngle`
  ;[1 1 1] Validate Rotation
  (if (`KismetMathLibrary.NearlyEqual_FloatFloat` (`self.CurrentRotationAngle`) (`self.CorrectRotationAngle`) 1.0)
    (set `self.isCorrect` true)
    (`/Game/Blueprints/Actors/Interaction/Puzzles/BP_PuzzleCircuitBoard.ValidatePuzzle` (`self.CircuitBoard`))
    (else
      (set `self.isCorrect` false))))

(fn `getNextRotationAngle`
  (returns (rotationAngle :type "Float (double-precision)"))
  (bind _currentrotationangle (`self.CurrentRotationAngle`))
  (if (== _currentrotationangle 0.0)
    (return 90.0)
    (elif (== _currentrotationangle 90.0)
      (return 180.0)
      (elif (== _currentrotationangle 180.0)
        (return 270.0)
        (elif (== _currentrotationangle 270.0)
          (return 360.0)
          (elif (== _currentrotationangle 360.0)
            (set `self.CurrentRotationAngle` 0.0)
            (return 90.0)))))))

(fn `UserConstructionScript`
  (`parent.UserConstructionScript`))