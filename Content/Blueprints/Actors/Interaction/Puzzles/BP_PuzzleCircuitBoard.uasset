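; Circuit board puzzle actor built from six child pipe actors that must all be rotated to their correct angles.
; BeginPlay configures each pipe's angles and visible segments, hands it a board reference, then reapplies tagged actor visibility if already solved.
; ValidatePuzzle checks every pipe; success saves solved state in the game instance, completes the task, swaps tagged actors, returns from BP_BlendTriggerVolume, opens tagged locked doors and later closes panel doors.
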(event `self.ReceiveBeginPlay`
  ;[0.2993 0.9446 1] Comment
  (`self.SetPipeVariableValues`)
  (bind _ashi_game_instance (cast `/Game/Blueprints/HI_GameInstance` (`GameplayStatics.GetGameInstance`)))
  (bind _hassolved (`/Game/Blueprints/HI_GameInstance.GetHasSolved` _ashi_game_instance (`self.HasSolvedVariable`)))
  (if _hassolved
    (`/Game/Blueprints/HI_GameInstance.HideActorsByTag` _ashi_game_instance (`self.HideActorsTag`) false)
    (`/Game/Blueprints/HI_GameInstance.ShowActorsByTag` _ashi_game_instance (`self.ShowActorsTag`))))

(event `ValidatePuzzle`
  ;[0.2923 0.4469 0.2033] Validate Puzzle
  (if (not (`self.isSolved`))
    (set `self.isSolved` true)
    (for _array_element (`self.PipesArray`)
      (if (not (`/Game/Blueprints/Actors/Interaction/Puzzles/BP_Interaction_Pipe.isCorrect` _array_element))
        (set `self.isSolved` false)))
    (if (`self.isSolved`)
      (bind _ashi_game_instance (cast `/Game/Blueprints/HI_GameInstance` (`GameplayStatics.GetGameInstance`)))
      (`/Game/Blueprints/HI_GameInstance.SetHasSolved` _ashi_game_instance (`self.HasSolvedVariable`) true)
      (`/Game/Blueprints/HI_GameInstance.TaskComplete` _ashi_game_instance)
      (`/Game/Blueprints/HI_GameInstance.ShowMessageUI` _ashi_game_instance (`self.SuccessMessage`))
      (`/Game/Blueprints/HI_GameInstance.HideActorsByTag` _ashi_game_instance (`self.HideActorsTag`) false)
      (`/Game/Blueprints/HI_GameInstance.ShowActorsByTag` _ashi_game_instance (`self.ShowActorsTag`))
      (bind _returnvalue (`GameplayStatics.GetActorOfClass` "/Game/Blueprints/Cameras/BP_BlendTriggerVolume.BP_BlendTriggerVolume_C"))
      (`/Game/Blueprints/Cameras/BP_BlendTriggerVolume.ReturnToCharacter` _returnvalue)
      (bind _outactors (`GameplayStatics.GetAllActorsOfClassWithTag` "/Game/Blueprints/Actors/Interaction/BP_DoorLockedByID.BP_DoorLockedByID_C" (`self.OpenDoorTag`)))
      (for _array_element_2 _outactors
        (`/Game/Blueprints/Actors/Interaction/BP_DoorLockedByID.OpenDoor` _array_element_2))
      (`KismetSystemLibrary.Delay` 2.0)
      (bind _outactors_2 (`GameplayStatics.GetAllActorsOfClassWithTag` "/Game/Blueprints/Actors/Interaction/BP_Interaction_Door_Open.BP_Interaction_Door_Open_C" (`self.PanelDoorTag`)))
      (for _array_element_3 _outactors_2
        (`/Game/Blueprints/Actors/Interaction/BP_Interaction_Door_Open.CloseDoor` _array_element_3)))))

(event `SetPipeVariableValues`
  (bind _pipesarray (`self.PipesArray`))
  ;[1 1 1] Comment
  (for _array_element (`self.PipesArray`)
    (`KismetArrayLibrary.Array_RemoveItem` (`self.PipesArray`) _array_element))
  (bind _asbp_interaction_pipe (cast `/Game/Blueprints/Actors/Interaction/Puzzles/BP_Interaction_Pipe` (`ChildActorComponent.ChildActor` (`self.BP_Interaction_Pipe0`))))
  (`KismetArrayLibrary.Array_Add` _pipesarray _asbp_interaction_pipe)
  (bind _asbp_interaction_pipe_2 (cast `/Game/Blueprints/Actors/Interaction/Puzzles/BP_Interaction_Pipe` (`ChildActorComponent.ChildActor` (`self.BP_Interaction_Pipe1`))))
  (`KismetArrayLibrary.Array_Add` _pipesarray _asbp_interaction_pipe_2)
  (bind _asbp_interaction_pipe_3 (cast `/Game/Blueprints/Actors/Interaction/Puzzles/BP_Interaction_Pipe` (`ChildActorComponent.ChildActor` (`self.BP_Interaction_Pipe2`))))
  (`KismetArrayLibrary.Array_Add` _pipesarray _asbp_interaction_pipe_3)
  (bind _asbp_interaction_pipe_4 (cast `/Game/Blueprints/Actors/Interaction/Puzzles/BP_Interaction_Pipe` (`ChildActorComponent.ChildActor` (`self.BP_Interaction_Pipe3`))))
  (`KismetArrayLibrary.Array_Add` _pipesarray _asbp_interaction_pipe_4)
  (bind _asbp_interaction_pipe_5 (cast `/Game/Blueprints/Actors/Interaction/Puzzles/BP_Interaction_Pipe` (`ChildActorComponent.ChildActor` (`self.BP_Interaction_Pipe4`))))
  (`KismetArrayLibrary.Array_Add` _pipesarray _asbp_interaction_pipe_5)
  (bind _asbp_interaction_pipe_6 (cast `/Game/Blueprints/Actors/Interaction/Puzzles/BP_Interaction_Pipe` (`ChildActorComponent.ChildActor` (`self.BP_Interaction_Pipe5`))))
  (`KismetArrayLibrary.Array_Add` _pipesarray _asbp_interaction_pipe_6)
  (`self.SetupPuzzle`))

(event `SetupPuzzle`
  ;[0.6237 0.03868 1] Comment
  (for (_array_element _array_index) (`self.PipesArray`)
    (set `/Game/Blueprints/Actors/Interaction/Puzzles/BP_Interaction_Pipe.CircuitBoard` self _array_element)
    (if (== _array_index 0)
      (`self.SetupPipe` _array_element (`self.Pipe0_StartAngle`) (`self.Pipe0_CorrectAngle`) (`self.Pipe0_Top`) (`self.Pipe0_Right`) (`self.Pipe0_Bottom`) (`self.Pipe0_Left`))
      (`/Game/Blueprints/Actors/Interaction/Puzzles/BP_Interaction_Pipe.SetupPipe` _array_element)
      (elif (== _array_index 1)
        (`self.SetupPipe` _array_element (`self.Pipe1_StartAngle`) (`self.Pipe1_CorrectAngle`) (`self.Pipe1_Top`) (`self.Pipe1_Right`) (`self.Pipe1_Bottom`) (`self.Pipe1_Left`))
        (`/Game/Blueprints/Actors/Interaction/Puzzles/BP_Interaction_Pipe.SetupPipe` _array_element)
        (elif (== _array_index 2)
          (`self.SetupPipe` _array_element (`self.Pipe2_StartAngle`) (`self.Pipe2_CorrectAngle`) (`self.Pipe2_Top`) (`self.Pipe2_Right`) (`self.Pipe2_Bottom`) (`self.Pipe2_Left`))
          (`/Game/Blueprints/Actors/Interaction/Puzzles/BP_Interaction_Pipe.SetupPipe` _array_element)
          (elif (== _array_index 3)
            (`self.SetupPipe` _array_element (`self.Pipe3_StartAngle`) (`self.Pipe3_CorrectAngle`) (`self.Pipe3_Top`) (`self.Pipe3_Right`) (`self.Pipe3_Bottom`) (`self.Pipe3_Left`))
            (`/Game/Blueprints/Actors/Interaction/Puzzles/BP_Interaction_Pipe.SetupPipe` _array_element)
            (elif (== _array_index 4)
              (`self.SetupPipe` _array_element (`self.Pipe4_StartAngle`) (`self.Pipe4_CorrectAngle`) (`self.Pipe4_Top`) (`self.Pipe4_Right`) (`self.Pipe4_Bottom`) (`self.Pipe4_Left`))
              (`/Game/Blueprints/Actors/Interaction/Puzzles/BP_Interaction_Pipe.SetupPipe` _array_element)
              (elif (== _array_index 5)
                (`self.SetupPipe` _array_element (`self.Pipe5_StartAngle`) (`self.Pipe5_CorrectAngle`) (`self.Pipe5_Top`) (`self.Pipe5_Right`) (`self.Pipe5_Bottom`) (`self.Pipe5_Left`))
                (`/Game/Blueprints/Actors/Interaction/Puzzles/BP_Interaction_Pipe.SetupPipe` _array_element)))))))))

(fn `SetupPipe`
  (params (PipeRef :type "/Game/Blueprints/Actors/Interaction/Puzzles/BP_Interaction_Pipe Object Reference") (CurrentRotationAngle :type "Float (double-precision)") (CorrectRotationAngle :type "Float (double-precision)") (ShowTop :type Boolean) (ShowRight :type Boolean) (ShowBottom :type Boolean) (ShowLeft :type Boolean))
  (`|ExecutionSequence`
    (:`then_0`
      (set `/Game/Blueprints/Actors/Interaction/Puzzles/BP_Interaction_Pipe.CurrentRotationAngle` CurrentRotationAngle PipeRef))
    (:`then_1`
      (set `/Game/Blueprints/Actors/Interaction/Puzzles/BP_Interaction_Pipe.CorrectRotationAngle` CorrectRotationAngle PipeRef))
    (:`then_2`
      (set `/Game/Blueprints/Actors/Interaction/Puzzles/BP_Interaction_Pipe.showPipeTop` ShowTop PipeRef))
    (:`then_3`
      (set `/Game/Blueprints/Actors/Interaction/Puzzles/BP_Interaction_Pipe.showPipeRight` ShowRight PipeRef))
    (:`then_4`
      (set `/Game/Blueprints/Actors/Interaction/Puzzles/BP_Interaction_Pipe.showPipeBottom` ShowBottom PipeRef))
    (:`then_5`
      (set `/Game/Blueprints/Actors/Interaction/Puzzles/BP_Interaction_Pipe.showPipeLeft` ShowLeft PipeRef))
    (:`then_6`
      (set `/Game/Blueprints/Actors/Interaction/Puzzles/BP_Interaction_Pipe.isCorrect` (== CurrentRotationAngle CorrectRotationAngle) PipeRef))))

(fn `UserConstructionScript`)