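; Clickable button for the spark plug puzzle, toggling between pressed and unpressed, with a material swap and a beep on press.
; Each click checks every button instance's pressed state against its ButtonValue until the game instance records the puzzle as solved.
; On success it completes the task, greens pressed buttons, disables BP_PuzzleSparkPlug actors, swaps tagged actor visibility, returns to the character and starts a timer.
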(event `self.ReceiveBeginPlay`
  (if (`self.isPressed`)
    (`self.PressButton`))
  (`parent.ReceiveBeginPlay`))

(event `/Game/Blueprints/Interfaces/BPI_Interaction.MouseClick`
  (bind _ashi_game_instance (cast `/Game/Blueprints/HI_GameInstance` (`GameplayStatics.GetGameInstance`)))
  (if (not (`/Game/Blueprints/HI_GameInstance.hasSolvedSparkPlugPuzzle` _ashi_game_instance))
    (if (`self.isPressed`)
      (`self.ResetButton`)
      (else
        (`self.PressButton`)))
    (set `self.isSolved` true)
    (bind _outactors (`GameplayStatics.GetAllActorsOfClass` "BP_Interaction_Sparkplug_C"))
    (for _array_element _outactors
      (if (`/Game/Blueprints/Actors/Interaction/Puzzles/BP_Interaction_Sparkplug.isPressed` _array_element)
        (bind _buttonvalue (`/Game/Blueprints/Actors/Interaction/Puzzles/BP_Interaction_Sparkplug.ButtonValue` _array_element))
        ;[1 1 1] if pressed, must equal 1
        (if (not (== _buttonvalue 1))
          ;[1 1 1] set to not solved
          (set `self.isSolved` false :!label _label))
        (else
          ;[1 1 1] if not pressed, must equal 0
          (if (not (== _buttonvalue 0))
            (goto _label)))))
    (if (`self.isSolved`)
      (`self.PuzzleSolved`))))

(event `/Game/Blueprints/Interfaces/BPI_Interaction.Interact`)

(event `PressButton`
  (`PrimitiveComponent.SetMaterial` (`self.Cube`) 1 "/Game/ModSci_Engineer/Materials/Lights/MI_Light_Red2.MI_Light_Red2")
  (set `self.isPressed` true)
  (`GameplayStatics.SpawnSoundAtLocation` "/Game/Audio/beep_03_Cue.beep_03_Cue" (`SceneComponent.K2_GetComponentLocation` (`self.Cube`)) (struct) 1.0 1.0 0.0 "/Game/Blueprints/SA_WalkAway.SA_WalkAway" null))

(event `ResetButton`
  (`PrimitiveComponent.SetMaterial` (`self.Cube`) 1 "/Game/ModularSpaceStation/Materials/MI_MSS_SpaceStation_1.MI_MSS_SpaceStation_1")
  (set `self.isPressed` false))

(event `SolvedButton`
  (`PrimitiveComponent.SetMaterial` (`self.Cube`) 1 "/Engine/EngineDebugMaterials/VertexColorViewMode_GreenOnly.VertexColorViewMode_GreenOnly"))

(event `PuzzleSolved`
  (bind _ashi_game_instance (cast `/Game/Blueprints/HI_GameInstance` (`GameplayStatics.GetGameInstance`)))
  (set `/Game/Blueprints/HI_GameInstance.hasSolvedSparkPlugPuzzle` true _ashi_game_instance)
  (`/Game/Blueprints/HI_GameInstance.TaskComplete` _ashi_game_instance)
  (bind _outactors (`GameplayStatics.GetAllActorsOfClass` "/Game/Blueprints/Actors/Interaction/Puzzles/BP_PuzzleSparkPlug.BP_PuzzleSparkPlug_C"))
  (for _array_element _outactors
    (`PrimitiveComponent.SetMaterial` (`/Game/Blueprints/Actors/Interaction/Puzzles/BP_PuzzleSparkPlug.StatusIndicator` _array_element) 1 "/Engine/EngineDebugMaterials/VertexColorViewMode_GreenOnly.VertexColorViewMode_GreenOnly"))
  (bind _outactors_2 (`GameplayStatics.GetAllActorsOfClass` "/Game/Blueprints/Actors/Interaction/Puzzles/BP_PuzzleSparkPlug.BP_PuzzleSparkPlug_C"))
  (for _array_element_2 _outactors_2
    (set `/Game/Blueprints/Actors/Interaction/BP_Interaction.ShowOutline` false _array_element_2)
    (set `/Game/Blueprints/Actors/Interaction/BP_Interaction.canInteract` false _array_element_2)
    (set `/Game/Blueprints/Actors/Interaction/BP_Interaction.ShowOutline` false _array_element_2)
    (`SceneComponent.SetVisibility` (`/Game/Blueprints/Actors/Interaction/BP_Interaction.Cube` _array_element_2) false false))
  (bind _outactors_3 (`GameplayStatics.GetAllActorsOfClass` "BP_Interaction_Sparkplug_C"))
  (for _array_element_3 _outactors_3
    (if (`/Game/Blueprints/Actors/Interaction/Puzzles/BP_Interaction_Sparkplug.isPressed` _array_element_3)
      (`self.SolvedButton` _array_element_3)))
  (`/Game/Blueprints/HI_GameInstance.ShowActorsByTag` _ashi_game_instance "sparkplugSolved")
  (`/Game/Blueprints/HI_GameInstance.HideActorsByTag` _ashi_game_instance "sparkplugRequired" false)
  (bind _returnvalue (`GameplayStatics.GetActorOfClass` "/Game/Blueprints/Cameras/BP_BlendTriggerVolume.BP_BlendTriggerVolume_C"))
  (`/Game/Blueprints/Cameras/BP_BlendTriggerVolume.ReturnToCharacter` _returnvalue)
  (`/Game/Blueprints/HI_GameInstance.BeginTimer` _ashi_game_instance))

(fn `UserConstructionScript`
  (`parent.UserConstructionScript`))