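; Interaction actor that starts the tram sequence when the player interacts with it.
; Its Interact event casts the game instance to HI_GameInstance and calls MoveTramSequence, leaving the sequence itself to that class.
; Unconnected leftover nodes for blending to the tram camera, moving BP_Tram, hiding the character and returning the view remain in the graph but never run.
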(event `/Game/Blueprints/Interfaces/BPI_Interaction.Interact`
  (bind _ashi_game_instance (cast `/Game/Blueprints/HI_GameInstance` (`GameplayStatics.GetGameInstance`)))
  (`/Game/Blueprints/HI_GameInstance.MoveTramSequence` _ashi_game_instance))

(fn `UserConstructionScript`
  (`parent.UserConstructionScript`))