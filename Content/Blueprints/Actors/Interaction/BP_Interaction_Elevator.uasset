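; Elevator actor that carries its mesh vertically between four preset floor heights.
; MoveElevator rejects requests while moving or to the same floor, resolves start and end heights via GetFloorLocation, starts the animation and immediately records the new current floor.
; AnimateElevatorMovement lerps the mesh's relative Z on a timeline while a door sound plays.
; During travel it hides the outline and interact option on the BP_AccessElevatorButtons actor found in the level.
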(event `AnimateElevatorMovement`
  (params (Start :type "Float (double-precision)") (Destination :type "Float (double-precision)"))
  (set `self.isMoving` true)
  (bind _returnvalue (`GameplayStatics.GetActorOfClass` "/Game/Blueprints/Actors/Interaction/BP_AccessElevatorButtons.BP_AccessElevatorButtons_C"))
  (set `/Game/Blueprints/Actors/Interaction/BP_Interaction.ShowOutline` false _returnvalue)
  (set `/Game/Blueprints/Actors/Interaction/BP_Interaction.ShowInteractOption` false _returnvalue)
  (bind _returnvalue_2 (`GameplayStatics.SpawnSound2D` "/Game/Audio/large_door_open_long.large_door_open_long" 1.0 1.0 0.0 null))
  (bind (_direction _newtrack_0) (`Timeline|Timeline_0` :`NewTime` 4.0 :!via `PlayFromStart`)
    (:`Update`
      (`SceneComponent.K2_SetRelativeLocation` (`self.StaticMesh`) (`KismetMathLibrary.MakeVector` 0.0 0.0 (`KismetMathLibrary.Lerp` Start Destination _newtrack_0)) false false))
    (:`Finished`
      (set `self.isMoving` false)
      (set `/Game/Blueprints/Actors/Interaction/BP_Interaction.ShowOutline` true _returnvalue)
      (set `/Game/Blueprints/Actors/Interaction/BP_Interaction.ShowInteractOption` true _returnvalue)
      (`AudioComponent.Stop` _returnvalue_2))))

(fn `GetFloorLocation`
  (params (FloorCurrent :type Integer) (FloorDestination :type Integer))
  (returns (LocationStart :type "Float (double-precision)") (LocationEnd :type "Float (double-precision)"))
  (bind _floorlocation1 (`self.FloorLocation1`))
  (bind _floorlocation2 (`self.FloorLocation2`))
  (bind _floorlocation4 (`self.FloorLocation4`))
  (bind _floorlocation3 (`self.FloorLocation3`))
  (if (== FloorCurrent 1)
    (if (== FloorDestination 1)
      (return _floorlocation1 _floorlocation1)
      (elif (== FloorDestination 2)
        (return _floorlocation1 _floorlocation2)
        (elif (== FloorDestination 3)
          (return _floorlocation1 _floorlocation3)
          (else
            (return _floorlocation1 _floorlocation4)))))
    (elif (== FloorCurrent 2)
      (if (== FloorDestination 1)
        (return _floorlocation2 _floorlocation1)
        (elif (== FloorDestination 2)
          (return _floorlocation2 _floorlocation2)
          (elif (== FloorDestination 3)
            (return _floorlocation2 _floorlocation3)
            (else
              (return _floorlocation2 _floorlocation4)))))
      (elif (== FloorCurrent 3)
        (if (== FloorDestination 1)
          (return _floorlocation3 _floorlocation1)
          (elif (== FloorDestination 2)
            (return _floorlocation3 _floorlocation2)
            (elif (== FloorDestination 3)
              (return _floorlocation3 _floorlocation3)
              (else
                (return _floorlocation3 _floorlocation4)))))
        (elif (== FloorDestination 1)
          (return _floorlocation4 _floorlocation1)
          (elif (== FloorDestination 2)
            (return _floorlocation4 _floorlocation2)
            (elif (== FloorDestination 3)
              (return _floorlocation4 _floorlocation3)
              (else
                (return _floorlocation4 _floorlocation4)))))))))

(fn `Move Elevator`
  (bind _destinationfloor (`self.DestinationFloor`))
  (if (`self.isMoving`)
    (`KismetSystemLibrary.PrintString` "Elevator is moving")
    (else
      (bind (_locationstart _locationend) (`self.GetFloorLocation` (`self.CurrentFloor`) _destinationfloor))
      (if (== _locationstart _locationend)
        (`KismetSystemLibrary.PrintString` "Same Floor")
        (else
          (`self.AnimateElevatorMovement` _locationstart _locationend)
          (`self.SetFloorLocations` (`KismetMathLibrary.Conv_IntToDouble` _destinationfloor)))))))

(fn `SetFloorLocations`
  (params (newCurrentFloor :type "Float (double-precision)"))
  (if (== newCurrentFloor 1.0)
    (set `self.CurrentFloor` 1)
    (elif (== newCurrentFloor 2.0)
      (set `self.CurrentFloor` 2)
      (elif (== newCurrentFloor 3.0)
        (set `self.CurrentFloor` 3)
        (elif (== newCurrentFloor 4.0)
          (set `self.CurrentFloor` 4))))))

(fn `UserConstructionScript`
  (`parent.UserConstructionScript`))