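; Interactable access card pickup that grants the player a door key from the access card generator.
; Interact only proceeds if the game instance has the key generator unlocked, then hides the card, shows a message and updates the key flags.
; It also resets every access card generator to its restricted display and un-presses all generate-key buttons.
; ShowCard and HideCard toggle mesh visibility, outline and interact option, with hiding also playing a pickup sound.
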(event `/Game/Blueprints/Interfaces/BPI_Interaction.Interact`
  (bind _ashi_game_instance (cast `/Game/Blueprints/HI_GameInstance` (`GameplayStatics.GetGameInstance`)))
  (if (`/Game/Blueprints/HI_GameInstance.hasUnlockedKeyGenerator` _ashi_game_instance)
    (`self.hideCard`)
    (`/Game/Blueprints/HI_GameInstance.ShowMessageUI` _ashi_game_instance "Door access granted")
    (set `/Game/Blueprints/HI_GameInstance.hasUnlockedKeyGenerator` false _ashi_game_instance)
    (set `/Game/Blueprints/HI_GameInstance.hasDoorKey` true _ashi_game_instance)
    (set `/Game/Blueprints/HI_GameInstance.hasGeneratedKey` false _ashi_game_instance)
    (bind _outactors (`GameplayStatics.GetAllActorsOfClass` "/Game/Blueprints/Actors/Interaction/BP_AccessCardGenerator.BP_AccessCardGenerator_C"))
    (for _array_element _outactors
      (`/Game/Blueprints/Actors/Interaction/BP_AccessCardGenerator.ResetButtons` _array_element)
      (`/Game/Blueprints/Actors/Interaction/BP_AccessCardGenerator.showAccessRestricted` _array_element))
    (bind _outactors_2 (`GameplayStatics.GetAllActorsOfClass` "/Game/Blueprints/Actors/Interaction/BP_Interaction_ButtonGenerateKey.BP_Interaction_ButtonGenerateKey_C"))
    (for _array_element_2 _outactors_2
      (`/Game/Blueprints/Actors/Interaction/BP_Interaction_ButtonGenerateKey.setUnPressed` _array_element_2))))

(fn `hideCard`
  (`SceneComponent.SetVisibility` (`self.Cube`) false false)
  (set `self.ShowOutline` false)
  (set `self.ShowInteractOption` false)
  (`Widget.SetVisibility` (`self.InteractWidget`) "Hidden")
  (`GameplayStatics.PlaySound2D` "/Engine/VREditor/Sounds/UI/Object_PickUp.Object_PickUp" 1.0 1.0 0.0 null null))

(fn `showCard`
  (`SceneComponent.SetVisibility` (`self.Cube`) true false)
  (set `self.ShowOutline` true)
  (set `self.ShowInteractOption` true))

(fn `UserConstructionScript`
  (`parent.UserConstructionScript`))