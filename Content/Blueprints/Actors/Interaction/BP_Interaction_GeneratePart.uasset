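; BP_Interaction_GeneratePart is an interactable, labeled with its PartName, that reveals the matching part for pickup.
; On Interact, it finds every BP_Interaction_PickupPart whose TextRender text equals PartName and shifts its Cube's relative Y location into place.
; A flag on HI_GameInstance, set on a match, blocks further generation while a part awaits pickup.
; Debug strings print both outcomes, and the parent BeginPlay call is disabled.
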(event `self.ReceiveBeginPlay`
  (`TextRenderComponent.K2_SetText` (`self.TextRender`) (`KismetTextLibrary.Conv_StringToText` (`self.PartName`))))

(event `/Game/Blueprints/Interfaces/BPI_Interaction.Interact`
  (bind _ashi_game_instance (cast `/Game/Blueprints/HI_GameInstance` (`GameplayStatics.GetGameInstance`)))
  (if (`/Game/Blueprints/HI_GameInstance.partGeneratedAndWaitingForPickup` _ashi_game_instance)
    (`KismetSystemLibrary.PrintString` "waiting for part to be picked up")
    (else
      (bind _outactors (`GameplayStatics.GetAllActorsOfClass` "/Game/Blueprints/Actors/Interaction/BP_Interaction_PickupPart.BP_Interaction_PickupPart_C"))
      (for _array_element _outactors
        (if (`KismetStringLibrary.EqualEqual_StrStr` (`KismetTextLibrary.Conv_TextToString` (`TextRenderComponent.Text` (`/Game/Blueprints/Actors/Interaction/BP_Interaction_PickupPart.TextRender` _array_element))) (`self.PartName`))
          (`SceneComponent.K2_SetRelativeLocation` (`/Game/Blueprints/Actors/Interaction/BP_Interaction.Cube` _array_element) (`KismetMathLibrary.MakeVector` 0.0 (`self.New Location Y`)) false false)
          (`KismetSystemLibrary.PrintString` "should be showing now")
          (set `/Game/Blueprints/HI_GameInstance.partGeneratedAndWaitingForPickup` true _ashi_game_instance))))))

(fn `UserConstructionScript`
  (`parent.UserConstructionScript`))