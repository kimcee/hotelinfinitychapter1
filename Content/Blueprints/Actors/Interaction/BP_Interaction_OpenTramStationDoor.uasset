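; Interaction Blueprint that opens the tram station door when the player holds the tram key.
; Interact checks the game instance's key flag, then either flags the main doors unlocked and calls MakeAccessGranted, or prints a key-needed message.
; MakeAccessGranted plays a sound, swaps open and closed door actors by tag, and opens the lockdown pillar.
; MakeAccessDenied swaps access indicators by tag but is never called here.
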(event `/Game/Blueprints/Interfaces/BPI_Interaction.Interact`
  (bind _ashi_game_instance (cast `/Game/Blueprints/HI_GameInstance` (`GameplayStatics.GetGameInstance`)))
  (if (`/Game/Blueprints/HI_GameInstance.hasTramKey` _ashi_game_instance)
    (set `/Game/Blueprints/HI_GameInstance.hasUnlockedMainDoors` true _ashi_game_instance)
    (`self.MakeAccessGranted`)
    (else
      (`KismetSystemLibrary.PrintString` "you need a tram door key"))))

(fn `MakeAccessDenied`
  (bind _outactors (`GameplayStatics.GetAllActorsWithTag` "doorAccessDenied"))
  (for _array_element _outactors
    (`SceneComponent.SetVisibility` (`Actor.RootComponent` _array_element) true false))
  (bind _outactors_2 (`GameplayStatics.GetAllActorsWithTag` "doorAccessGranted"))
  (for _array_element_2 _outactors_2
    (`SceneComponent.SetVisibility` (`Actor.RootComponent` _array_element_2) false false))
  (`KismetSystemLibrary.PrintString` "You must use your key again"))

(fn `MakeAccessGranted`
  (`GameplayStatics.PlaySound2D` "/Engine/VREditor/Sounds/UI/Enter_Play.Enter_Play" 1.0 1.0 0.0 null null)
  (bind _ashi_game_instance (cast `/Game/Blueprints/HI_GameInstance` (`GameplayStatics.GetGameInstance`)))
  (`/Game/Blueprints/HI_GameInstance.ShowActorsByTag` _ashi_game_instance "tramStationDoorIsOpen")
  (`/Game/Blueprints/HI_GameInstance.HideActorsByTag` _ashi_game_instance "tramStationDoorIsClosed" false)
  (bind _returnvalue (`GameplayStatics.GetActorOfClass` "/Game/Blueprints/Actors/Movement/BP_LockdownPillarsStutter.BP_LockdownPillarsStutter_C"))
  (`/Game/Blueprints/Actors/Movement/BP_LockdownPillarsStutter.OpenPillar` _returnvalue))

(fn `UserConstructionScript`
  (`parent.UserConstructionScript`))