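; Camera-focus helper that blends the player's view to a given camera and back to the character, with no overlap logic of its own.
; MoveToCamera sets IsFocused, hides the HUD and interact widget, enables mouse clicks, and disables movement and look input.
; ReturnToCharacter restores view, controls and character visibility but leaves both widgets hidden.
; Separate functions hide or show the player character.
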(fn `HideCharacter`
  (`self.SetActorHiddenInGame` (`GameplayStatics.GetPlayerCharacter` 0) true))

(fn `MoveToCamera`
  (params (Camera :type "CameraActor Object Reference"))
  (bind _returnvalue (`GameplayStatics.GetPlayerCharacter` 0))
  (bind _returnvalue_2 (`GameplayStatics.GetPlayerController` 0))
  (bind _asbp_hiplayer_char (cast `/Game/Blueprints/Characters/PC/BP_HIPlayerChar` (`GameplayStatics.GetPlayerCharacter` 0)))
  (if (`KismetSystemLibrary.IsValid` _asbp_hiplayer_char)
    (bind _asplayer_controller (cast `PlayerController` (`Pawn.GetController` _asbp_hiplayer_char)))
    (if (`KismetSystemLibrary.IsValid` _asplayer_controller)
      (`PlayerController.SetViewTargetWithBlend` _asplayer_controller Camera (`self.CameraBlendTime`) "VTBlend_Linear" 0.0 false)
      (bind _asbp_hiplayer_char_2 (cast `/Game/Blueprints/Characters/PC/BP_HIPlayerChar` _returnvalue))
      (`Widget.SetVisibility` (`/Game/Blueprints/Characters/PC/BP_HIPlayerChar.MainHUDRed` _asbp_hiplayer_char_2) "Hidden")
      (set `self.isFocused` true)
      (set `PlayerController.bShowMouseCursor` true _returnvalue_2)
      (set `PlayerController.bEnableClickEvents` true _returnvalue_2)
      (`ActorComponent.Deactivate` (`Character.CharacterMovement` _returnvalue))
      (`Controller.SetIgnoreLookInput` _returnvalue_2 true)
      (`Widget.SetVisibility` (`/Game/Blueprints/Characters/PC/BP_HIPlayerChar.InteractWidget` _asbp_hiplayer_char) "Hidden"))
    (else
      (`KismetSystemLibrary.PrintString` "Did not work"))))

(fn `ReturnToCharacter`
  (bind _returnvalue (`GameplayStatics.GetPlayerController` 0))
  (bind _returnvalue_2 (`GameplayStatics.GetPlayerCharacter` 0))
  (bind _asbp_hiplayer_char (cast `/Game/Blueprints/Characters/PC/BP_HIPlayerChar` (`GameplayStatics.GetPlayerCharacter` 0)))
  (if (`KismetSystemLibrary.IsValid` _asbp_hiplayer_char)
    (bind _asplayer_controller (cast `PlayerController` (`Pawn.GetController` _asbp_hiplayer_char)))
    (if (`KismetSystemLibrary.IsValid` _asplayer_controller)
      (set `self.isFocused` false)
      (`PlayerController.SetViewTargetWithBlend` _asplayer_controller _asbp_hiplayer_char (`self.CameraBlendTime`) "VTBlend_Linear" 0.0 false)
      (bind _asbp_hiplayer_char_2 (cast `/Game/Blueprints/Characters/PC/BP_HIPlayerChar` _returnvalue_2))
      (`Widget.SetVisibility` (`/Game/Blueprints/Characters/PC/BP_HIPlayerChar.MainHUDRed` _asbp_hiplayer_char_2) "Hidden")
      (set `PlayerController.bShowMouseCursor` false _returnvalue)
      (set `PlayerController.bEnableClickEvents` false _returnvalue)
      (`ActorComponent.Activate` (`Character.CharacterMovement` _returnvalue_2) false)
      (`Controller.ResetIgnoreLookInput` _returnvalue)
      (`self.SetActorHiddenInGame` _returnvalue_2 false))))

(fn `ShowCharacter`
  (`self.SetActorHiddenInGame` (`GameplayStatics.GetPlayerCharacter` 0) false))

(fn `UserConstructionScript`)