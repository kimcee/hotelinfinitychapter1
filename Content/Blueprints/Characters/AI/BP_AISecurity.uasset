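; BP_AISecurity is a hanging AI security sentry that watches for the player through overlap detection while powered.
; BeginPlay starts a looping hanging animation after a random delay and sets a repeating timer at a randomized interval.
; That timer briefly cuts power, hiding its spot and point lights, and overlaps during the outage trigger no alarm.
; Detection currently only prints debug messages, and a locked-versus-roaming branch is left unconnected.
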(event `self.ReceiveBeginPlay`
  ;[1 1 1] Event Begin Play: PowerFlicker
  (`KismetSystemLibrary.K2_SetTimerDelegate` (delegate `PowerFlicker`) (`KismetMathLibrary.RandomFloatInRange` 24.0 84.0) true)
  (`KismetSystemLibrary.Delay` (`KismetMathLibrary.RandomFloatInRange` 0.0 4.0))
  (`SkeletalMeshComponent.PlayAnimation` (`self.Mesh`) "/Game/Characters/Animations/A_HangingAI1.A_HangingAI1" true))

(event `PowerFlicker`
  (bind _spotlight (`self.SpotLight`))
  ;[1 1 1] Event Begin Play: PowerFlicker
  (bind _output_get (set `self.HasPower` false))
  (`SceneComponent.SetVisibility` _spotlight _output_get false)
  (`SceneComponent.SetVisibility` (`self.PointLight`) _output_get false)
  (`KismetSystemLibrary.Delay` (`KismetMathLibrary.RandomFloatInRange` 0.42 2.4))
  (bind _output_get_2 (set `self.HasPower` true))
  (`SceneComponent.SetVisibility` _spotlight _output_get_2 false)
  (`SceneComponent.SetVisibility` (`self.PointLight`) _output_get_2 false))

(event `self.ReceiveActorBeginOverlap`
  (params (OtherActor :type "Actor Object Reference"))
  ;[1 1 1] Alarm!
  (if (`self.HasPower`)
    (cast `/Game/Blueprints/Characters/PC/BP_HIPlayerChar` OtherActor)
    (`KismetSystemLibrary.PrintString` "Player Detected - Sound Alarms!")
    (else
      (`KismetSystemLibrary.PrintString` "No Power - Do Nothing"))))

(fn `UserConstructionScript`
  (`parent.UserConstructionScript`))