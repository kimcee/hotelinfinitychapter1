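; Player character for a puzzle game, handling movement, sprint, item-gated flashlight and journal, footsteps, death and respawn.
; BeginPlay creates the HUD, journal, death, pause, hint and admin widgets, which input events toggle.
; Interaction sends BPI_Interaction messages to overlapping actors or cursor hits.
; Pausing copies position and GameInstance progress flags into an existing save slot; save setup/loading at startup and the regen timer are disconnected.
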(event `self.ReceiveBeginPlay`
  ;[1 1 1] BeginPlay
  (`self.Initialize`)
  (`parent.ReceiveBeginPlay`)
  ;[1 1 1] Footsteps Effects
  (`Timeline|Footsteps` :!via `PlayFromStart`))

(event `TickRegen`
  (bind _currenthealth (`self.CurrentHealth`))
  ;[0.3767 1 0.37] Health & Stamina Regen:
  ; If Player is ALIVE w/o negative status effect
  (if (> _currenthealth 0)
    (`/Engine/EditorBlueprintResources/StandardMacros.IncrementInt` _currenthealth
      (:`  `
        (`/Engine/EditorBlueprintResources/StandardMacros.IncrementInt` (`self.CurrentStamina`))))
    (else
      (`KismetSystemLibrary.PrintString` "You dead"))))

(event `InputAction|Sprint`
  (params (Key :type "Key Structure"))
  (bind _charactermovement (`self.CharacterMovement`))
  ;[1 0.3581 0] Movement & View: INPUTS
  ;;[1 1 1] Sprint Toggle
  (:`Pressed`
    (set `self.isSprinting` true)
    (set `CharacterMovementComponent.MaxWalkSpeed` 1000.0 _charactermovement))
  (:`Released`
    (set `self.isSprinting` false)
    (set `CharacterMovementComponent.MaxWalkSpeed` 400.0 _charactermovement)))

(event `StartCameraShake`
  ;[1 0.3581 0] Movement & View: INPUTS
  ;;[1 0.2451 0.3812] Camera Shake (Sprint)
  (`PlayerController.ClientStartCameraShake` :`self` (`GameplayStatics.GetPlayerController` 0) :`Shake` "/Script/Engine.CameraShakeBase"))

(event `InputAxis|MoveForwardBackward`
  (params (AxisValue :type "Float (single-precision)"))
  (bind _returnvalue (`KismetMathLibrary.SelectFloat` 1.0 AxisValue (`self.isSprinting`)))
  ;[1 0.3581 0] Movement & View: INPUTS
  ;;[1 1 1] Move Forward / Backward (moving backwards is slower than moving forward)
  (if (`self.MovementLocked`)
    (`KismetSystemLibrary.PrintString` "Your Movement is LOCKED!")
    (else
      (`self.AddMovementInput` (`KismetMathLibrary.GetForwardVector` (`KismetMathLibrary.MakeRotator` 0.0 0.0 (.yaw (`self.K2_GetActorRotation`)))) (* (`KismetMathLibrary.SelectFloat` 1.0 0.3 (>= _returnvalue 0.0)) _returnvalue)))))

(event `StopCameraShake`
  ;[1 0.3581 0] Movement & View: INPUTS
  ;;[1 0.2451 0.3812] Camera Shake (Sprint)
  (`PlayerController.ClientStopCameraShake` (`GameplayStatics.GetPlayerController` 0) "/Script/Engine.CameraShakeBase" true))

(event `InputAction|Jump`
  (params (Key :type "Key Structure"))
  ;[1 0.3581 0] Movement & View: INPUTS
  ;;[1 1 1] Jumping
  (:`Pressed`
    (if (not (`self.MovementLocked`))
      (`self.Jump`)))
  (:`Released`
    (`self.StopJumping`)))

(event `InputAxis|StrafeLeftRight`
  (params (AxisValue :type "Float (single-precision)"))
  ;[1 0.3581 0] Movement & View: INPUTS
  ;;[1 1 1] Strafe
  (if (not (`self.MovementLocked`))
    (`self.AddMovementInput` (`KismetMathLibrary.GetRightVector` (`KismetMathLibrary.MakeRotator` 0.0 0.0 (.yaw (`self.K2_GetActorRotation`)))) AxisValue)))

(event `InputAction|Crouch`
  (params (Key :type "Key Structure"))
  ;[1 0.3581 0] Movement & View: INPUTS
  ;;[1 1 1] Crouching ?? Will decide how to do this later
  (:`Pressed`
    (if (`NavMovementComponent.IsCrouching` (`self.CharacterMovement`))
      _)))

(event `InputAxis|LookUpDown`
  (params (AxisValue :type "Float (single-precision)"))
  ;[1 0.3581 0] Movement & View: INPUTS
  ;;[1 1 1] Look / Turn
  (if (not (`self.MovementLocked`))
    (`self.AddControllerPitchInput` AxisValue)))

(event `InputAxis|TurnLeftRight`
  (params (AxisValue :type "Float (single-precision)"))
  ;[1 0.3581 0] Movement & View: INPUTS
  ;;[1 1 1] Look / Turn
  (if (not (`self.MovementLocked`))
    (`self.AddControllerYawInput` AxisValue)))

(event `InputAction|PlayerFlashLight`
  (params (Key :type "Key Structure"))
  ;[0.2525 0.4086 1] Flashlight
  (:`Pressed`
    (bind _ashi_game_instance (cast `/Game/Blueprints/HI_GameInstance` (`GameplayStatics.GetGameInstance`)))
    (if (`/Game/Blueprints/HI_GameInstance.hasFlashLight` _ashi_game_instance)
      (if (`SceneComponent.bVisible` (`self.SpotLight`))
        (`GameplayStatics.PlaySound2D` null 1.0 1.0 0.0 null null)
        (`SceneComponent.SetVisibility` (`self.SpotLight`) false false)
        (bind (_direction _alphaval) (`Timeline|AnimateFlashLightTL` :!via `Reverse` :!label _label)
          (:`Update`
            (`SceneComponent.K2_SetRelativeLocation` (`self.Flashlight`) (`KismetMathLibrary.MakeVector` 17.0 17.0 (`KismetMathLibrary.Lerp` 0.0 15.0 _alphaval)) false false)))
        (else
          (`|ExecutionSequence`
            (:`then_0`
              (`SceneComponent.SetVisibility` (`self.Flashlight`) true false))
            (:`then_1`
              (goto _label))
            (:`then_2`
              (`KismetSystemLibrary.Delay` 0.5)
              (`GameplayStatics.PlaySound2D` null 1.0 1.0 0.0 null null)
              (`SceneComponent.SetVisibility` (`self.SpotLight`) true false)))))
      (else
        (`KismetSystemLibrary.PrintString` "Find the flashlight")))))

(event `InputAction|PlayerToggleJournal`
  (params (Key :type "Key Structure"))
  ;[1 1 1] Journal Trigger
  (:`Pressed`
    (bind _ashi_game_instance (cast `/Game/Blueprints/HI_GameInstance` (`GameplayStatics.GetGameInstance`)))
    (if (`/Game/Blueprints/HI_GameInstance.hasJournal` _ashi_game_instance)
      (`self.ToggleJournal`)
      (else
        (`KismetSystemLibrary.PrintString` "Find the journal")))))

(event `InputAction|PlayerInitAdmin`
  (params (Key :type "Key Structure"))
  (bind _returnvalue (`GameplayStatics.GetPlayerController` 0))
  ;[1 0.04547 0.05169] Admin Toggle
  (:`Pressed`
    (`KismetSystemLibrary.PrintString` "Init Admin")
    (`/Engine/EditorBlueprintResources/StandardMacros.FlipFlop`
      (:`A`
        (`Widget.SetVisibility` (`self.AdminWidget`) "Visible")
        (set `self.isViewingWidget` true)
        (set `PlayerController.bShowMouseCursor` true _returnvalue))
      (:`B`
        (`Widget.SetVisibility` (`self.AdminWidget`) "Hidden")
        (set `self.isViewingWidget` false)
        (set `PlayerController.bShowMouseCursor` false _returnvalue)))))

(event `ToggleJournal`
  (bind _journalwidget (`self.JournalWidget`))
  ;[1 1 1] JournalToggle
  (`/Engine/EditorBlueprintResources/StandardMacros.FlipFlop`
    (:`A`
      (`Widget.SetVisibility` _journalwidget "Visible")
      (set `self.isViewingWidget` true))
    (:`B`
      (`Widget.SetVisibility` _journalwidget "Hidden")
      (set `self.isViewingWidget` false))))

(event `InputAction|PlayerExitFocus`
  (params (Key :type "Key Structure"))
  ;[1 1 1] Un-Focus Player
  (:`Pressed`
    (bind _returnvalue (`GameplayStatics.GetActorOfClass` "/Game/Blueprints/Cameras/BP_BlendTriggerVolume.BP_BlendTriggerVolume_C"))
    (if (`/Game/Blueprints/Cameras/BP_BlendTriggerVolume.isFocused` _returnvalue)
      (`/Game/Blueprints/Cameras/BP_BlendTriggerVolume.ReturnToCharacter` _returnvalue)
      (bind _ashi_game_instance (cast `/Game/Blueprints/HI_GameInstance` (`GameplayStatics.GetGameInstance`)))
      (`/Game/Blueprints/HI_GameInstance.HideActorsByTag` _ashi_game_instance "keyboardForComputer" false))))

(event `Key|V`
  (params (Key :type "Key Structure")))

(event `InputTouch` :consume false
  (params (Location :type "Vector Structure") (FingerIndex :type "ETouchIndex Enum"))
  ;[0.5562 1 0.42] Player Interact / no line trace
  (:`Pressed`
    (set `self.ImplementsActor` false :!label _label_2)
    (for _array_element (`self.GetOverlappingActors` "/Script/Engine.Actor")
      (if (`KismetSystemLibrary.DoesImplementInterface` _array_element "/Game/Blueprints/Interfaces/BPI_Interaction.BPI_Interaction_C")
        (message `/Game/Blueprints/Interfaces/BPI_Interaction.Interact` _array_element)
        (set `self.ImplementsActor` true)))
    (if (`self.ImplementsActor`)
      (set `self.ImplementsActor` false))))

(event `InputTouch` :consume false
  (params (Location :type "Vector Structure") (FingerIndex :type "ETouchIndex Enum"))
  (bind (_hitresult _returnvalue) (`PlayerController.GetHitResultUnderCursorForObjects` (`GameplayStatics.GetPlayerController` 0) (`|MakeArray` "ObjectTypeQuery2" :!type "EObjectTypeQuery Enum") true))
  (bind (_bblockinghit _binitialoverlap _time _distance _location _impactpoint _normal _impactnormal _physmat _hitactor) (`GameplayStatics.BreakHitResult` _hitresult))
  ;[1 1 1] Mouse Interaction
  (:`Pressed`
    (if _returnvalue :!label _label_3
      (if (and (`KismetSystemLibrary.IsValid` _hitactor) (`KismetSystemLibrary.DoesImplementInterface` _hitactor "/Game/Blueprints/Interfaces/BPI_Interaction.BPI_Interaction_C"))
        ;;[1 0.3765 0.9973] Mouse Click Events
        (message `/Game/Blueprints/Interfaces/BPI_Interaction.MouseClick` _hitactor)))))

(event `InputAction|PlayerMouseInteract`
  (params (Key :type "Key Structure"))
  ;[1 1 1] Mouse Interaction
  (:`Pressed`
    (goto _label_3)))

(event `InputAction|PlayerInteract`
  (params (Key :type "Key Structure"))
  ;[0.5562 1 0.42] Player Interact / no line trace
  (:`Pressed`
    (goto _label_2)))

(event `InputAction|PlayerPauseGame` :paused true
  (params (Key :type "Key Structure"))
  (bind _pausewidget (`self.PauseWidget`))
  ;[0.3205 0.1014 0.4811] Pause Game
  (:`Pressed`
    (`/Engine/EditorBlueprintResources/StandardMacros.FlipFlop` :!label _label_4
      (:`A`
        (`self.SaveGameState`)
        (`GameplayStatics.SetGamePaused` true)
        (`Widget.SetVisibility` _pausewidget "Visible"))
      (:`B`
        (`GameplayStatics.SetGamePaused` false)
        (`Widget.SetVisibility` _pausewidget "Hidden")))))

(event `KillPlayer`
  (bind _playerdiedwidget (`self.PlayerDiedWidget`))
  ;[1 0 0] Kill Player
  (if (not (`self.isPlayerDead`))
    (set `self.isPlayerDead` true)
    (`GameplayStatics.PlaySound2D` null 1.0 1.0 0.0 null null)
    (set `self.isViewingWidget` true)
    (`Widget.SetVisibility` _playerdiedwidget "Visible")
    (`WidgetBlueprintLibrary.SetInputMode_GameAndUIEx` (`GameplayStatics.GetPlayerController` 0) _playerdiedwidget "DoNotLock" false)))

(event `Resume`
  ;[0.3205 0.1014 0.4811] Pause Game
  (goto _label_4))

(event `RespawnPlayer`
  (params (Player :type "Character Object Reference"))
  ;[0.1181 0.7986 1] Respawn Player Event
  (`self.K2_SetActorTransform` (`self.RespawnTransform`))
  (set `self.isViewingWidget` false)
  (set `self.isPlayerDead` false)
  (`Widget.SetVisibility` (`self.PlayerDiedWidget`) "Hidden")
  (`WidgetBlueprintLibrary.SetInputMode_GameOnly` (`GameplayStatics.GetPlayerController` 0)))

(event `Key|T`
  (params (Key :type "Key Structure"))
  ;[0 0 0] Debug Player Death and Respawn
  (:`Pressed`
    (`KismetSystemLibrary.PrintString` "Spawn Point Set")
    (`self.SetSpawnPoint`)))

(event `Key|K`
  (params (Key :type "Key Structure"))
  ;[0 0 0] Debug Player Death and Respawn
  (:`Pressed`
    (`KismetSystemLibrary.PrintString` "Kill Player")
    (`self.KillPlayer`)))

(fn `Initialize`
  (`|ExecutionSequence`
    (:`then_1`
      ;[0.1676 0.7132 1] Widgets
      (bind _returnvalue (`|CreateWidget` "/Game/UI/W_MainHUD.W_MainHUD_C"))
      (bind _output_get (set `self.MainHUDRed` _returnvalue))
      (`UserWidget.AddToViewport` _output_get 0)
      (`Widget.SetVisibility` _output_get "Hidden"))
    (:`then_2`
      (bind _returnvalue_2 (`|CreateWidget` "/Game/UI/WBP_Journal.WBP_Journal_C"))
      (bind _output_get_2 (set `self.JournalWidget` _returnvalue_2))
      (`UserWidget.AddToViewport` _output_get_2 0)
      (`Widget.SetVisibility` _output_get_2 "Hidden"))
    (:`then_3`
      (bind _returnvalue_3 (`|CreateWidget` "/Game/UI/WBP_DeathScreen.WBP_DeathScreen_C"))
      (bind _output_get_3 (set `self.PlayerDiedWidget` _returnvalue_3))
      (`UserWidget.AddToViewport` _output_get_3 0)
      (`Widget.SetVisibility` _output_get_3 "Hidden"))
    (:`then_4`
      (bind _returnvalue_4 (`|CreateWidget` "/Game/UI/WBP_Interact.WBP_Interact_C"))
      (bind _output_get_4 (set `self.InteractWidget` _returnvalue_4))
      (`UserWidget.AddToViewport` _output_get_4 0)
      (`Widget.SetVisibility` _output_get_4 "Hidden"))
    (:`then_5`
      (bind _returnvalue_5 (`|CreateWidget` "/Game/UI/WBP_PauseScreen.WBP_PauseScreen_C"))
      (bind _output_get_5 (set `self.PauseWidget` _returnvalue_5))
      (`UserWidget.AddToViewport` _output_get_5 0)
      (`Widget.SetVisibility` _output_get_5 "Hidden"))
    (:`then_6`
      (bind _returnvalue_6 (`|CreateWidget` "/Game/UI/WBP_UserHints.WBP_UserHints_C"))
      (bind _output_get_6 (set `self.UserHintsWidget` _returnvalue_6))
      (`UserWidget.AddToViewport` _output_get_6 0))
    (:`then_7`
      (bind _returnvalue_7 (`|CreateWidget` "/Game/UI/WBP_Admin.WBP_Admin_C"))
      (bind _output_get_7 (set `self.AdminWidget` _returnvalue_7))
      (`UserWidget.AddToViewport` _output_get_7 0)
      (`Widget.SetVisibility` _output_get_7 "Hidden"))))

(fn `LoadGame`
  (bind _returnvalue (`GameplayStatics.LoadGameFromSlot` (`self.SaveGameSlot`)))
  (bind _ashi_save_game (cast `/Game/Blueprints/HI_SaveGame` _returnvalue))
  (bind _output_get (set `self.HISaveGame` _ashi_save_game))
  (bind _ashi_game_instance (cast `/Game/Blueprints/HI_GameInstance` (`GameplayStatics.GetGameInstance`)))
  (`|ExecutionSequence`
    (:`then_0`
      (set `/Game/Blueprints/HI_GameInstance.hasFlashLight` (`/Game/Blueprints/HI_SaveGame.hasFlashLight` _output_get) _ashi_game_instance))
    (:`then_1`
      (set `/Game/Blueprints/HI_GameInstance.hasPryingTool` (`/Game/Blueprints/HI_SaveGame.hasPryingTool` _output_get) _ashi_game_instance))
    (:`then_2`
      (set `/Game/Blueprints/HI_GameInstance.hasKeyboard` (`/Game/Blueprints/HI_SaveGame.hasKeyboard` _output_get) _ashi_game_instance))
    (:`then_3`
      (set `/Game/Blueprints/HI_GameInstance.hasDoorKey` (`/Game/Blueprints/HI_SaveGame.hasDoorKey` _output_get) _ashi_game_instance))
    (:`then_4`
      (set `/Game/Blueprints/HI_GameInstance.hasTramKey` (`/Game/Blueprints/HI_SaveGame.hasTramKey` _output_get) _ashi_game_instance))
    (:`then_5`
      (set `/Game/Blueprints/HI_GameInstance.hasSolvedElectricalPanel` (`/Game/Blueprints/HI_SaveGame.hasSolvedElectricalPanel` _output_get) _ashi_game_instance))
    (:`then_6`
      (set `/Game/Blueprints/HI_GameInstance.hasSolvedElevatorPuzzle` (`/Game/Blueprints/HI_SaveGame.hasSolvedElevatorPuzzle` _output_get) _ashi_game_instance))
    (:`then_7`
      (set `/Game/Blueprints/HI_GameInstance.hasSolvedSecurityLasers` (`/Game/Blueprints/HI_SaveGame.hasSolvedSecurityLasers` _output_get) _ashi_game_instance))
    (:`then_8`
      (set `/Game/Blueprints/HI_GameInstance.hasSolvedSparkPlugPuzzle` (`/Game/Blueprints/HI_SaveGame.hasSolvedSparkPlugPuzzle` _output_get) _ashi_game_instance))
    (:`then_9`
      (`self.K2_SetActorTransform` (`/Game/Blueprints/HI_SaveGame.PlayerPosition` _output_get)))))

(fn `PlayFootstep`
  (params (Landing :type Boolean))
  (bind _returnvalue (`self.K2_GetActorLocation`))
  (bind _charactermovement (`self.CharacterMovement`))
  (bind (_outhit _returnvalue_2) (`KismetSystemLibrary.LineTraceSingle` _returnvalue (+ _returnvalue (0.0 0.0 -100.0)) "TraceTypeQuery1"))
  (if _returnvalue_2
    (if Landing
      (bind (_bblockinghit _binitialoverlap _time _distance _location _impactpoint _normal _impactnormal _physmat) (`GameplayStatics.BreakHitResult` _outhit))
      (bind _returnvalue_3 (select `EPhysicalSurface` (`PhysicalMaterial.SurfaceType` _physmat) :!type "SoundBase Object Reference"))
      (`GameplayStatics.PlaySoundAtLocation` _returnvalue_3 _impactpoint (struct) 1.0 0.0 0.0 null null null null)
      (else
        (`GameplayStatics.PlaySoundAtLocation` _returnvalue_3 _impactpoint (struct) (`KismetMathLibrary.MapRangeUnclamped` (`KismetMathLibrary.VSize` (`self.GetVelocity`)) (`CharacterMovementComponent.MaxWalkSpeedCrouched` _charactermovement) (`CharacterMovementComponent.MaxWalkSpeed` _charactermovement) 0.25 0.5) 0.0 0.0 null null null null)))))

(fn `PlayFootstepConditional`
  (bind _charactermovement (`self.CharacterMovement`))
  (if (and (> (`KismetMathLibrary.VSize` (`MovementComponent.Velocity` _charactermovement)) 10.0) (not (`NavMovementComponent.IsFalling` _charactermovement)))
    (`self.PlayFootstep` false)))

(fn `SaveGameState`
  (bind _hisavegame (`self.HISaveGame`))
  (bind _returnvalue (`GameplayStatics.DoesSaveGameExist` (`self.SaveGameSlot`)))
  (if _returnvalue
    (bind _ashi_game_instance (cast `/Game/Blueprints/HI_GameInstance` (`GameplayStatics.GetGameInstance`)))
    (`|ExecutionSequence`
      (:`then_0`
        (`self.SetSpawnPoint`)
        (set `/Game/Blueprints/HI_SaveGame.PlayerPosition` (`self.RespawnTransform`) _hisavegame))
      (:`then_1`
        (set `/Game/Blueprints/HI_SaveGame.hasFlashLight` (`/Game/Blueprints/HI_GameInstance.hasFlashLight` _ashi_game_instance) _hisavegame))
      (:`then_2`
        (set `/Game/Blueprints/HI_SaveGame.hasPryingTool` (`/Game/Blueprints/HI_GameInstance.hasPryingTool` _ashi_game_instance) _hisavegame))
      (:`then_3`
        (set `/Game/Blueprints/HI_SaveGame.hasKeyboard` (`/Game/Blueprints/HI_GameInstance.hasKeyboard` _ashi_game_instance) _hisavegame))
      (:`then_4`
        (set `/Game/Blueprints/HI_SaveGame.hasDoorKey` (`/Game/Blueprints/HI_GameInstance.hasDoorKey` _ashi_game_instance) _hisavegame))
      (:`then_5`
        (set `/Game/Blueprints/HI_SaveGame.hasTramKey` (`/Game/Blueprints/HI_GameInstance.hasTramKey` _ashi_game_instance) _hisavegame))
      (:`then_6`
        (set `/Game/Blueprints/HI_SaveGame.hasSolvedElectricalPanel` (`/Game/Blueprints/HI_GameInstance.hasSolvedElectricalPanel` _ashi_game_instance) _hisavegame))
      (:`then_7`
        (set `/Game/Blueprints/HI_SaveGame.hasSolvedElevatorPuzzle` (`/Game/Blueprints/HI_GameInstance.hasSolvedElevatorPuzzle` _ashi_game_instance) _hisavegame))
      (:`then_8`
        (set `/Game/Blueprints/HI_SaveGame.hasSolvedSecurityLasers` (`/Game/Blueprints/HI_GameInstance.hasSolvedSecurityLasers` _ashi_game_instance) _hisavegame))
      (:`then_9`
        (set `/Game/Blueprints/HI_SaveGame.hasSolvedSparkPlugPuzzle` (`/Game/Blueprints/HI_GameInstance.hasSolvedSparkPlugPuzzle` _ashi_game_instance) _hisavegame))
      (:`then_10`
        (`GameplayStatics.SaveGameToSlot` null (`self.SaveGameSlot`))))))

(fn `SetSpawnPoint`
  (set `self.RespawnTransform` (`self.GetTransform`)))

(fn `UserConstructionScript`
  (`parent.UserConstructionScript`))