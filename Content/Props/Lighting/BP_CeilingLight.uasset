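; BP_CeilingLight is a ceiling light prop that flickers off briefly at intervals during play.
; On BeginPlay it starts a looping timer whose interval is randomized once per instance, so separate lights flicker out of sync.
; Each flicker swaps the mesh to an unlit material and hides the rect light, then restores both after a short random delay.
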(event `self.ReceiveBeginPlay`
  ;[1 1 1] Begin Play: Light Flicker
  (`KismetSystemLibrary.K2_SetTimerDelegate` (delegate `LightFlicker`) (`KismetMathLibrary.RandomFloatInRange` 24.0 84.0) true 24.0 4.0))

(event `LightFlicker`
  (bind _sm_ceilinglight (`self.SM_CeilingLight`))
  (bind _rectceilinglight (`self.RectCeilingLight`))
  ;[1 1 1] Begin Play: Light Flicker
  (`PrimitiveComponent.SetMaterial` _sm_ceilinglight 0 "/Game/Props/Lighting/M_LightsOff.M_LightsOff")
  (`SceneComponent.SetVisibility` _rectceilinglight false false)
  (`KismetSystemLibrary.Delay` (`KismetMathLibrary.RandomFloatInRange` 0.24 2.4))
  (`PrimitiveComponent.SetMaterial` _sm_ceilinglight 0 "/Game/Props/Lighting/M_LightsOn.M_LightsOn")
  (`SceneComponent.SetVisibility` _rectceilinglight true false))

(fn `UserConstructionScript`)