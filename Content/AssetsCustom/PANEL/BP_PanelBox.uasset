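; Wire panel puzzle actor with an optional cover, where recolouring wires completes two conduits.
; SetWireCombo swaps a wire's material slot and calls CheckWireCombo, which tests each conduit's goal slots for light green.
; When both conduits are complete it calls EventOnSuccess.
; Interact and EventOnSuccess are empty here; the cover-drop, UI creation and door auto-open logic is disconnected and never runs.
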(event `self.Interact`
  (params (Caller :type "Actor Object Reference"))
  ;[1 1 1] Panel Interaction
)

(event `EventOnSuccess`
  ;[1 1 1] On Panel Re-wire Success
)

(fn `CheckWireCombo`
  (params (`Conduit Number` :type Integer))
  (switch `int` `Conduit Number`
    (:`0`
      (if (== (`PrimitiveComponent.GetMaterial` (`self.SM_WirePanel`) (`|GetArrayItem` (`self.GoalWireCombosConduitA`))) "/Game/ThirdParty/BigCompanyArchViz/Materials/MI_LightGreen.MI_LightGreen")
        (set `self.ConduitAComplete?` true)
        (`GameplayStatics.PlaySound2D` "/Game/Audio/beep_03.beep_03" 1.0 1.0 0.0 null null)
        (else
          (set `self.ConduitAComplete?` false))))
    (:`1`
      (if (and (== (`PrimitiveComponent.GetMaterial` (`self.SM_WirePanel`) (`|GetArrayItem` (`self.GoalWireCombosConduitB`))) "/Game/ThirdParty/BigCompanyArchViz/Materials/MI_LightGreen.MI_LightGreen") (== (`PrimitiveComponent.GetMaterial` (`self.SM_WirePanel`) (`|GetArrayItem` (`self.GoalWireCombosConduitB`) 1)) "/Game/ThirdParty/BigCompanyArchViz/Materials/MI_LightGreen.MI_LightGreen"))
        (set `self.ConduitBComplete?` true)
        (`GameplayStatics.PlaySound2D` "/Game/Audio/beep_03.beep_03" 1.0 1.0 0.0 null null)
        (else
          (set `self.ConduitBComplete?` false)))))
  (if (and (`self.ConduitAComplete?`) (`self.ConduitBComplete?`))
    (`self.EventOnSuccess`))
  (return))

(fn `SetWireCombo`
  (params (WireIndex :type Integer) (`Wire Color` :type "MaterialInterface Object Reference") (`Conduit Number` :type Integer))
  (`PrimitiveComponent.SetMaterial` (`self.SM_WirePanel`) WireIndex `Wire Color`)
  (`self.CheckWireCombo` `Conduit Number`)
  (`GameplayStatics.PlaySound2D` null 1.0 1.0 0.0 null null)
  (return))

(fn `UserConstructionScript`
  (`SceneComponent.SetVisibility` (`self.panel_COVER`) (`self.ShowCover?`) false))